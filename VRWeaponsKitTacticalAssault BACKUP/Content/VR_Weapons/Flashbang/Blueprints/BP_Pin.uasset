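; BP_Pin is the VR flashbang's safety pin, removable by hand or teeth, with actor collision disabled at BeginPlay.
; Pickup snaps it to the hand's PullRingSocket, mirroring it for the left hand, while pulling it out of a Teeth-tagged overlap detaches it with physics.
; Both removal paths play sound, start lever-pressure haptics and set PinRemoved on BPFlashbang, arming it to explode on release.
; Drop detaches it with physics; other interaction functions are stubs.
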(event `self.ReceiveBeginPlay`
  (`self.SetActorEnableCollision` false) ; Disable pin collision until flashbang has been grabbed
)

(event `/Game/VR_Weapons/Pawn/Blueprints/PickupActorInterface.Drop`
  (`PrimitiveComponent.SetSimulatePhysics` (`self.Pin`) true)
  (`self.K2_DetachFromActor` "KeepWorld" "KeepWorld" "KeepWorld"))

(event `self.Overlap.OnComponentBeginOverlap`
  (params (OverlappedComponent :type "PrimitiveComponent Object Reference") (OtherActor :type "Actor Object Reference") (OtherComp :type "PrimitiveComponent Object Reference") (OtherBodyIndex :type Integer) (bFromSweep :type Boolean) (SweepResult :type "HitResult Structure (by ref)"))
  ;[0 0 0] Remove pin with teeth
  (if (`ActorComponent.ComponentHasTag` OtherComp "Teeth")
    (`/Engine/EditorBlueprintResources/StandardMacros.DoOnce` false
      (:`Completed`
        (`KismetSystemLibrary.PrintString` "Overlapped" true true (struct :`R` 0.329358 :`G` 1.0 :`B` 0.518123 :`A` 1.0) 8.0)
        (`GameplayStatics.PlaySoundAtLocation` "/Game/VR_Weapons/Flashbang/Audio/Flashbang_pin_remove_teeth_Cue.Flashbang_pin_remove_teeth_Cue" (`SceneComponent.K2_GetComponentLocation` (`self.Overlap`)) (struct) 1.0 1.0 0.0 "/Game/VR_Weapons/Global/Audio/Small_object_Attenuation.Small_object_Attenuation" null null)))))

(event `self.Overlap.OnComponentEndOverlap`
  (params (OverlappedComponent :type "PrimitiveComponent Object Reference") (OtherActor :type "Actor Object Reference") (OtherComp :type "PrimitiveComponent Object Reference") (OtherBodyIndex :type Integer))
  ;[0 0 0] Remove pin with teeth
  (if (`ActorComponent.ComponentHasTag` OtherComp "Teeth")
    (`/Game/VR_Weapons/Flashbang/Blueprints/BP_Flashbang.Lever Pressure Haptics` (`self.BP_Flashbang`)) ; lever pressure rumble
    (set `/Game/VR_Weapons/Flashbang/Blueprints/BP_Flashbang.pin removed` true (`self.BP_Flashbang`)) ; tell BP_flashbang the pin has been removed\nand the flashbang is ready to explode when released
    (`GameplayStatics.PlaySoundAtLocation` "/Game/VR_Weapons/Flashbang/Audio/Flashbang_pin_remove_Cue.Flashbang_pin_remove_Cue" (`self.K2_GetActorLocation`) (struct) 1.0 1.0 0.0 "/Game/VR_Weapons/Global/Audio/Small_object_Attenuation.Small_object_Attenuation" null null)
    (`PrimitiveComponent.SetSimulatePhysics` (`self.Pin`) true)
    (`self.K2_DetachFromActor` "KeepWorld" "KeepWorld" "KeepWorld")))

(fn `GripHandGuard`
  (params (Hand :type "/Game/VR_Weapons/Pawn/Blueprints/BP_MotionController Object Reference"))
  (returns (HandguardGrabbed :type Boolean))
  (return false))

(fn `InsertMagazine`
  (params (OverlappedComponent :type "PrimitiveComponent Object Reference") (WeaponType :type "/Game/VR_Weapons/Pawn/Blueprints/E_WeaponType Enum" :default "NewEnumerator0"))
  (returns (`Magazine Compatible` :type Boolean) (`Weapon Mesh` :type "StaticMeshComponent Object Reference") (`Weapon Actor` :type "/Game/VR_Weapons/Global/Blueprints/BP_Gun Object Reference"))
  (return false null null))

(fn `Pickup`
  (params (Hand :type "EControllerHand Enum" :default "Left") (`Grip or grab` :type "/Game/VR_Weapons/Pawn/Blueprints/E_GrabType Enum" :default "NewEnumerator1") (Actor :type "/Game/VR_Weapons/Pawn/Blueprints/BP_MotionController Object Reference") (AttachTo :type "SceneComponent Object Reference"))
  (returns (WeaponType :type "/Game/VR_Weapons/Pawn/Blueprints/E_WeaponType Enum") (GunGrabbed :type Boolean))
  (`/Game/VR_Weapons/Pawn/Blueprints/BP_MotionController.RumbleController` Actor "/Game/VR_Weapons/Pawn/Haptics/Haptics_single.Haptics_single" 1.0 false) ; pin removal click
  (`/Game/VR_Weapons/Flashbang/Blueprints/BP_Flashbang.Lever Pressure Haptics` (`self.BP_Flashbang`)) ; lever pressure rumble
  (set `/Game/VR_Weapons/Pawn/Blueprints/BP_MotionController.Engage` true Actor) ; change the hand animation to engage
  (set `/Game/VR_Weapons/Flashbang/Blueprints/BP_Flashbang.pin removed` true (`self.BP_Flashbang`)) ; tell BP_flashbang the pin has been removed\nand the flashbang is ready to explode when released
  (`SceneComponent.SetWorldScale3D` (`self.Pin`) (`KismetMathLibrary.SelectVector` (1.0 1.0 -1.0) (1.0 1.0 1.0) (`|EnumEquality` Hand "Left"))) ; Flip if grabbed by left hand
  (`PrimitiveComponent.SetSimulatePhysics` (`self.Pin`) false)
  (`SceneComponent.K2_AttachToComponent` (`self.K2_GetRootComponent`) AttachTo "PullRingSocket" "SnapToTarget" "SnapToTarget" "KeepWorld" true)
  (`SceneComponent.K2_SetRelativeRotation` (`self.Pullring`) (struct :`Pitch` 45.0 :`Yaw` 43.0 :`Roll` -55.84) false false)
  (`GameplayStatics.PlaySoundAtLocation` "/Game/VR_Weapons/Flashbang/Audio/Flashbang_pin_remove_Cue.Flashbang_pin_remove_Cue" (`self.K2_GetActorLocation`) (struct) 1.0 1.0 0.0 "/Game/VR_Weapons/Global/Audio/Small_object_Attenuation.Small_object_Attenuation" null null)
  (return "NewEnumerator2" false))

(fn `PullTrigger`
  (returns (Fired :type Boolean))
  (return false))

(fn `UserConstructionScript`)