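; BP_Shotgun_cartridge is a VR shotgun round that the player grabs by hand and loads into BP_Shotgun.
; Pickup snaps it to a hand socket on a grab only, Drop detaches it with physics, and the other weapon functions are stubs.
; When its capsule overlaps a shotgun with magazine space, it triggers the shotgun's insert response, haptics and sound.
; After a short delay it adds the round, releases the hand and destroys itself.
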(event `self.Capsule.OnComponentBeginOverlap`
  (params (OverlappedComponent :type "PrimitiveComponent Object Reference") (OtherActor :type "Actor Object Reference") (OtherComp :type "PrimitiveComponent Object Reference") (OtherBodyIndex :type Integer) (bFromSweep :type Boolean) (SweepResult :type "HitResult Structure (by ref)"))
  (bind _asbp_shotgun (cast `/Game/VR_Weapons/Guns/Shotgun/Blueprints/BP_Shotgun` OtherActor))
  (bind _asbp_magazine_shotgun (cast `/Game/VR_Weapons/Guns/Shotgun/Blueprints/BP_Magazine_shotgun` (`/Game/VR_Weapons/Global/Blueprints/BP_Gun.Magazine` _asbp_shotgun)))
  ;[0 0 0] Check there is space for a new round
  (if (< (`/Game/VR_Weapons/Global/Blueprints/BP_Magazine.Rounds` _asbp_magazine_shotgun) (`/Game/VR_Weapons/Guns/Shotgun/Blueprints/BP_Magazine_shotgun.Mag max capacity` _asbp_magazine_shotgun))
    (`/Game/VR_Weapons/Guns/Shotgun/Blueprints/BP_Shotgun.Round inserted` _asbp_shotgun) ; play cartirdge elevator anim
    (bind _bp_motion_controller (`self.BP motion controller`)
      (:`then`
        ;[0 0 0] cartridge insert sound and vibration
        (`/Game/VR_Weapons/Pawn/Blueprints/BP_MotionController.RumbleController` _bp_motion_controller "/Game/VR_Weapons/Pawn/Haptics/Haptics_single.Haptics_single" 0.75 false))
      (:`else`
        _))
    (`GameplayStatics.PlaySoundAtLocation` "/Game/VR_Weapons/Guns/Shotgun/Audio/Shotgun_cartridge_insert_Cue.Shotgun_cartridge_insert_Cue" (`self.K2_GetActorLocation`) (struct) 1.0 1.0 0.0 "/Game/VR_Weapons/Global/Audio/Small_object_Attenuation.Small_object_Attenuation" "/Game/VR_Weapons/Global/Audio/WeaponConcurrency.WeaponConcurrency" null)
    (`KismetSystemLibrary.Delay` 0.1)
    (`/Game/VR_Weapons/Guns/Shotgun/Blueprints/BP_Magazine_shotgun.Add round` _asbp_magazine_shotgun) ; Call function to add a new round to the magazine
    (bind _bp_motion_controller_2 (`self.BP motion controller`)
      (:`then`
        ;[0 0 0] update hand to stop gripping
        (set `/Game/VR_Weapons/Pawn/Blueprints/BP_MotionController.Engage` false _bp_motion_controller_2)
        (set `/Game/VR_Weapons/Pawn/Blueprints/BP_MotionController.Weapon` "NewEnumerator0" _bp_motion_controller_2))
      (:`else`
        _))
    (`self.K2_DestroyActor`)))

(event `/Game/VR_Weapons/Pawn/Blueprints/PickupActorInterface.Drop`
  (`PrimitiveComponent.SetSimulatePhysics` (`self.SM_Cartridge`) true)
  (`self.K2_DetachFromActor` "KeepWorld" "KeepWorld" "KeepWorld"))

(fn `GripHandGuard`
  (params (Hand :type "/Game/VR_Weapons/Pawn/Blueprints/BP_MotionController Object Reference"))
  (returns (HandguardGrabbed :type Boolean))
  (return false))

(fn `InsertMagazine`
  (params (OverlappedComponent :type "PrimitiveComponent Object Reference") (WeaponType :type "/Game/VR_Weapons/Pawn/Blueprints/E_WeaponType Enum" :default "NewEnumerator0"))
  (returns (`Magazine Compatible` :type Boolean) (`Weapon Mesh` :type "StaticMeshComponent Object Reference") (`Weapon Actor` :type "/Game/VR_Weapons/Global/Blueprints/BP_Gun Object Reference"))
  (return false null null))

(fn `Pickup`
  (params (Hand :type "EControllerHand Enum" :default "Left") (`Grip or grab` :type "/Game/VR_Weapons/Pawn/Blueprints/E_GrabType Enum" :default "NewEnumerator1") (Actor :type "/Game/VR_Weapons/Pawn/Blueprints/BP_MotionController Object Reference") (AttachTo :type "SceneComponent Object Reference"))
  (returns (WeaponType :type "/Game/VR_Weapons/Pawn/Blueprints/E_WeaponType Enum") (GunGrabbed :type Boolean))
  (set `self.BP motion controller` Actor)
  (set `self.Hand mesh` AttachTo)
  (if (`|EnumEquality` `Grip or grab` "NewEnumerator1")
    (`PrimitiveComponent.SetSimulatePhysics` (`self.SM_Cartridge`) false)
    (`SceneComponent.K2_AttachToComponent` (`self.K2_GetRootComponent`) (`self.Hand mesh`) "Shotgun_CartridgeGripSocket" "SnapToTarget" "SnapToTarget" "SnapToTarget" true)
    (set `/Game/VR_Weapons/Pawn/Blueprints/BP_MotionController.Engage` true (`local.Actor`)) ; Set hand to engage to update \nblendspace anim
    (return "NewEnumerator6" false)))

(fn `PullTrigger`
  (returns (Fired :type Boolean))
  (return false))

(fn `UserConstructionScript`)