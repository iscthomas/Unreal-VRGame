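; Handgun silencer pickup for VR that snaps onto a compatible BP_Handgun.
; Overrides the parent's collision overlap to attach to the barrel mesh's Silencer socket rather than the gun mesh.
; Attachment requires a matching weapon type, a Silencer-tagged collider, a ready silencer and no silencer already fitted.
; It detaches from the hand, notifies the gun, plays a sound and clears the right-hand AnimBP's silencer grip state.
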(event `self.Collision.OnComponentBeginOverlap`
  (params (OverlappedComponent :type "PrimitiveComponent Object Reference") (OtherActor :type "Actor Object Reference") (OtherComp :type "PrimitiveComponent Object Reference") (OtherBodyIndex :type Integer) (bFromSweep :type Boolean) (SweepResult :type "HitResult Structure (by ref)"))
  (bind _bp_motioncontroller (`self.BP_MotionController`))
  ;[0 0 0] Overide parent to attach to barrel instead of gun mesh
  (bind _asbp_handgun (cast `/Game/VR_Weapons/Guns/Handgun/Blueprints/BP_Handgun` OtherActor))
  (if (and (`|EnumEquality` (`/Game/VR_Weapons/Global/Blueprints/BP_Gun.Weapon` _asbp_handgun) (`self.Weapon Type`)) (`ActorComponent.ComponentHasTag` OtherComp "Silencer") (`self.Silencer ready`) (== (`/Game/VR_Weapons/Global/Blueprints/BP_Gun.Silencer` _asbp_handgun) false))
    (set `self.BP_gun` _asbp_handgun) ; create bp gun reference
    (`self.K2_DetachFromActor` "KeepWorld" "KeepWorld" "KeepWorld") ; detach from hand
    (bind _returnvalue (`SceneComponent.K2_AttachToComponent` (`self.Silencer`) (`/Game/VR_Weapons/Guns/Handgun/Blueprints/BP_Handgun.SM_handgun_barrel` _asbp_handgun) "Silencer" "SnapToTarget" "SnapToTarget" "SnapToTarget" true)) ; attach to gun
    (if _returnvalue
      (`/Game/VR_Weapons/Global/Blueprints/BP_Gun.Silencer attached` (`self.BP_gun`))
      (`GameplayStatics.PlaySoundAtLocation` "/Game/VR_Weapons/Global/Audio/Silencer_attach_Cue.Silencer_attach_Cue" (`SceneComponent.K2_GetComponentLocation` (`self.Collision`)) (struct) 1.0 1.0 0.0 "/Game/VR_Weapons/Global/Audio/Small_object_Attenuation.Small_object_Attenuation" null null)
      ;;[0 0 0] Update AnimBP grip state
      (`/Engine/EditorBlueprintResources/StandardMacros.IsValid` _bp_motioncontroller
        (:`Is Valid`
          (bind _asright_hand_anim_bp (cast `/Game/VR_Weapons/Pawn/Mannequin/Animations/RightHand_AnimBP` (`SkeletalMeshComponent.GetAnimInstance` (`/Game/VR_Weapons/Pawn/Blueprints/BP_MotionController.HandMesh` _bp_motioncontroller))))
          (set `/Game/VR_Weapons/Pawn/Mannequin/Animations/RightHand_AnimBP.Silencer` false _asright_hand_anim_bp))))))

(fn `UserConstructionScript`
  (`parent.UserConstructionScript`)
  (set `self.Weapon Type` "NewEnumerator4"))