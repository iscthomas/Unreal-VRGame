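; VR flashbang grenade: grabbed by hand, armed by pulling a spawned pin, detonates after a delay when dropped unpinned, or on BeginPlay if flagged.
; The blast uses sphere overlaps and line traces, bouncing traces off walls indoors, to reach the player and living AI.
; AI get distance-scaled stuns; players get a screen flash (widget or post-process, by device) and muffled ear ringing.
; Effects include particles, light, decal, radial impulse and ejected lever.
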(event `self.ReceiveBeginPlay`
  (bind _returnvalue (`self.K2_GetActorLocation`))
  (bind _particle_effect (`self.Particle effect`))
  (bind _enemy_character (`self.Enemy character`))
  (bind _blast_radius (`self.blast radius`))
  (bind _target_pawn_class (`self.Target pawn class`))
  (bind _flash_intensity (`self.Flash intensity`))
  (bind _flashbang_grenade (`self.Flashbang_grenade`))
  (bind _lever (`self.Lever`))
  (bind _returnvalue_2 (`SceneComponent.K2_GetComponentLocation` (`self.Flashbang_grenade`)))
  (bind _overlappingactors (`PrimitiveComponent.GetOverlappingActors` (`self.Player collision sphere`) _target_pawn_class))
  (bind _returnvalue_3 (`PrimitiveComponent.WasRecentlyRendered` (`self.Flashbang_grenade`) 0.1))
  (bind _output (`|GetArrayItem` _overlappingactors))
  (bind _returnvalue_4 (+ (`KismetMathLibrary.MapRangeClamped` (`KismetMathLibrary.Vector_Distance` (`self.K2_GetActorLocation` _enemy_character) (`self.K2_GetActorLocation`)) (/ _blast_radius 2.0) _blast_radius (`self.Stun duration max`) (`self.Stun duration min`)) (`KismetMathLibrary.RandomFloatInRange` -2.0 2.0)))
  ;[0 0 0] Setup
  (`|ExecutionSequence`
    (:`then_0`
      (bind _returnvalue_5 (`|SpawnActorFromClass` "/Game/VR_Weapons/Flashbang/Blueprints/BP_Pin.BP_Pin_C" (`self.GetTransform`) "Undefined" "OverrideRootScale" null self null)) ; Spawn pin actor that can be removed from flashbang before throwing
      (bind _output_get (set `self.BP_pin` _returnvalue_5))
      (`SceneComponent.K2_AttachToComponent` (`self.K2_GetRootComponent` _output_get) (`self.Flashbang_grenade`) "Pin" "SnapToTarget" "SnapToTarget" "SnapToTarget" true)
      (`PrimitiveComponent.SetSimulatePhysics` (`self.Flashbang_grenade`) (`self.Start simulating physics`)))
    (:`then_1`
      (`KismetSystemLibrary.Delay` (`KismetMathLibrary.RandomFloatInRange` 1.0 2.0))
      (if (`self.explode on event begin play`)
        ;[0 0 0] Release
        (`|ExecutionSequence` :!label _label
          (:`then_0`
            (`KismetSystemLibrary.Delay` 0.2)
            (`SceneComponent.K2_DetachFromComponent` (`self.Lever`) "KeepWorld" "KeepWorld" "KeepWorld" true)
            (bind (_direction _rotation) (`Timeline|Lever detach animation` :!via `PlayFromStart`)
              (:`Update`
                (`SceneComponent.K2_SetRelativeRotation` _lever (`KismetMathLibrary.MakeRotator` 0.0 (`KismetMathLibrary.Lerp` 0.0 215.0 _rotation)) false false))
              (:`Finished`
                (`PrimitiveComponent.SetSimulatePhysics` _lever true)
                (add `PrimitiveComponent.OnComponentHit` (`self.Lever`) (delegate `Hit`)))))
          (:`then_1`
            (`/Engine/EditorBlueprintResources/StandardMacros.DoOnce` false
              (:`Completed`
                (`KismetSystemLibrary.Delay` (`self.delay`)) ; delay before bang
                (`|ExecutionSequence`
                  (:`then_0`
                    ;[0 0 0] Check nearby player
                    (if (and (> (`KismetArrayLibrary.Array_Length` _overlappingactors) 0) (== (`GameplayStatics.GetObjectClass` _output) _target_pawn_class))
                      (bind _output_get_2 (set `self.nearby pawn` _output))
                      (`KismetSystemLibrary.PrintString` (`KismetSystemLibrary.GetDisplayName` _output) true true (struct :`R` 0.985801 :`B` 1.0 :`A` 1.0) 0.5)
                      (bind _asplayer_head (cast `/Game/VR_Weapons/Pawn/Blueprints/PlayerHead` _output_get_2)
                        (:`then`
                          (bind _output_get_3 (set `self.Player head` (`/Game/VR_Weapons/Pawn/Blueprints/PlayerHead.HeadSphere` _asplayer_head))) ; Head Sphere collision is the target
                          (bind _outhit (`KismetSystemLibrary.LineTraceSingle` :`Start` (`SceneComponent.K2_GetComponentLocation` (`self.Flashbang_grenade`)) :`End` (`SceneComponent.K2_GetComponentLocation` _output_get_3) :`TraceChannel` (`self.Trace channel`) :`DrawDebugType` (select `bool` (`self.Debug mode`) :`true` "ForDuration" :!type "EDrawDebugTrace Enum") :`TraceColor` (struct :`R` 1.0 :`G` 0.237876 :`A` 1.0))) ; line trace to player's head to check if anything is blocking the flashbang
                          (if (== (`.HitActor` (`GameplayStatics.BreakHitResult` _outhit)) (`self.nearby pawn`))
                            (`KismetSystemLibrary.PrintString` "Flashbang heard" true true (struct :`R` 0.070988 :`G` 1.0 :`A` 1.0) 4.0)
                            (set `self.Flashbang heard` true))
                          (bind _hit (`self.LineTraceEnvironment` (750.0 0.0 0.0))) ; X
                          (bind _hit_2 (`self.LineTraceEnvironment` (0.0 750.0 0.0))) ; Y
                          (bind _hit_3 (`self.LineTraceEnvironment` (0.0 0.0 750.0))) ; Z
                          (bind _hit_4 (`self.LineTraceEnvironment` (-750.0 0.0 0.0))) ; -X
                          (bind _hit_5 (`self.LineTraceEnvironment` (0.0 -750.0 0.0))) ; -Y
                          (bind _hit_6 (`self.LineTraceEnvironment` (0.0 0.0 -750.0))) ; -Z
                          (if (and _hit_3 _hit_2 _hit _hit_4 _hit_5 _hit_6)
                            (for _ (range (`self.Close proximity bounces`))
                              (bind _line_trace_hit_actor (`self.Bounce line traces inside` (`SceneComponent.K2_GetComponentLocation` (`self.Player head`)) (`self.nearby pawn`))) ; Bounce line traces off walls/objects in an attempt to reach player
                              (if _line_trace_hit_actor
                                (bind _output_get_4 (set `self.Close interior proximity` true))
                                (`KismetSystemLibrary.PrintString` "Bounce Reached Player" _output_get_4 _output_get_4 (struct :`R` 0.006027 :`G` 1.0 :`A` 1.0) 4.0))))
                          (if (or (`self.Flashbang heard`) (`self.Close interior proximity`))
                            (`KismetSystemLibrary.PrintString` (`KismetStringLibrary.Conv_BoolToString` _returnvalue_3) true true (struct :`R` 1.0 :`G` 0.381992 :`A` 1.0) 4.0)
                            (`KismetSystemLibrary.PrintString` "Player looking at flashbang" _returnvalue_3 _returnvalue_3 (struct :`R` 0.129183 :`G` 1.0 :`A` 1.0))
                            (if (or _returnvalue_3 (`self.Close interior proximity`))
                              (`KismetSystemLibrary.Delay` 0.03)
                              (bind _oculus_quest (`/Game/VR_Weapons/Global/Blueprints/GlobalFunctions.CheckDevice`))
                              (if _oculus_quest
                                (bind _asmotion_controller_pawn (cast `/Game/VR_Weapons/Pawn/Blueprints/MotionControllerPawn` (`GameplayStatics.GetPlayerPawn` 0))
                                  (:`then`
                                    (bind _asflashbang_widget (cast `/Game/VR_Weapons/Global/FlashbangWidget` (`WidgetComponent.GetUserWidgetObject` (`/Game/VR_Weapons/Pawn/Blueprints/MotionControllerPawn.ScreenFlashWidget` _asmotion_controller_pawn)))
                                      (:`then`
                                        (`/Game/VR_Weapons/Global/FlashbangWidget.WhiteFlash` _asflashbang_widget)
                                        (`KismetSystemLibrary.Delay` (`KismetMathLibrary.MapRangeClamped` (`self.explosion distance`) 0.3 1.0 (`self.Stun duration min`) (`self.Stun duration max`)))
                                        (`/Game/VR_Weapons/Global/FlashbangWidget.FadeBack` _asflashbang_widget))
                                      (:`CastFailed`
                                        (`KismetSystemLibrary.PrintString` "CAST to widget FAILED" true true (struct :`R` 1.0 :`G` 0.039531 :`A` 1.0) 3.0))))
                                  (:`CastFailed`
                                    (`KismetSystemLibrary.PrintString` "CAST to motion controller FAILED" true true (struct :`R` 1.0 :`G` 0.039531 :`A` 1.0) 3.0)))
                                (else
                                  (`KismetMaterialLibrary.SetScalarParameterValue` "/Game/VR_Weapons/Flashbang/Materials/MPC_Flashbang.MPC_Flashbang" "FlashBrightness" _flash_intensity)
                                  (`KismetMaterialLibrary.SetScalarParameterValue` "/Game/VR_Weapons/Flashbang/Materials/MPC_Flashbang.MPC_Flashbang" "FlashOverallEffect" _flash_intensity)
                                  (`KismetSystemLibrary.Delay` (`KismetMathLibrary.MapRangeClamped` (`self.explosion distance`) 0.3 1.0 (`self.Stun duration min`) (`self.Stun duration max`))) ; delay before fading from blindness back to normal
                                  (bind (_direction_2 _alpha) (`Timeline|Fade` :!via `PlayFromStart`)
                                    (:`Update`
                                      (`KismetMaterialLibrary.SetScalarParameterValue` "/Game/VR_Weapons/Flashbang/Materials/MPC_Flashbang.MPC_Flashbang" "FlashOverallEffect" (`KismetMathLibrary.Lerp` (`self.Flash intensity`) 0.0 _alpha)))))))))
                        (:`CastFailed`
                          (`KismetSystemLibrary.PrintString` "cast failed")))))
                  (:`then_1`
                    ;[0 0 0] Check enemy AI pawn
                    (for _array_element (`PrimitiveComponent.GetOverlappingActors` (`self.Player collision sphere`) (`self.Target AI class`))
                      (`/Engine/EditorBlueprintResources/StandardMacros.IsValid` _array_element
                        (:`Is Valid`
                          (bind _asenemy_character (cast `/Game/VR_Weapons/AI/Enemy_character` _array_element))
                          (if (not (`/Game/VR_Weapons/AI/Enemy_character.dead` _asenemy_character))
                            (set `self.Enemy character` _asenemy_character)
                            (bind _outhit_2 (`KismetSystemLibrary.LineTraceSingle` :`Start` (`self.K2_GetActorLocation`) :`End` (`SceneComponent.GetSocketLocation` (`Character.Mesh` _asenemy_character) "Head") :`TraceChannel` (`self.Trace channel`) :`DrawDebugType` (select `bool` (`self.Debug mode`) :`true` "ForDuration" :!type "EDrawDebugTrace Enum") :`TraceColor` (struct :`R` 1.0 :`G` 0.237876 :`A` 1.0))) ; line trace to player to AI's head to check if anything is blocking the flashbang
                            (if (== (`.HitActor` (`GameplayStatics.BreakHitResult` _outhit_2)) (`self.Enemy character`))
                              (`/Game/VR_Weapons/AI/Enemy_character.Stunned event` _enemy_character _returnvalue_4 :!label _label_2)
                              (`KismetSystemLibrary.PrintString` (`KismetStringLibrary.Conv_DoubleToString` _returnvalue_4))
                              (else
                                (bind _hit_7 (`self.LineTraceEnvironment` (750.0 0.0 0.0))) ; X
                                (bind _hit_8 (`self.LineTraceEnvironment` (0.0 750.0 0.0))) ; Y
                                (bind _hit_9 (`self.LineTraceEnvironment` (0.0 0.0 750.0))) ; Z
                                (bind _hit_10 (`self.LineTraceEnvironment` (-750.0 0.0 0.0))) ; -X
                                (bind _hit_11 (`self.LineTraceEnvironment` (0.0 -750.0 0.0))) ; -Y
                                (bind _hit_12 (`self.LineTraceEnvironment` (0.0 0.0 -750.0))) ; -Z
                                (if (and _hit_9 _hit_8 _hit_7 _hit_10 _hit_11 _hit_12)
                                  (bind _actor_hit (`self.Try to reach AI`))
                                  (if _actor_hit
                                    (goto _label_2))))))))))
                  (:`then_2`
                    ;[0 0 0] Particle and sound effects
                    (`GameplayStatics.PlaySoundAtLocation` "/Game/VR_Weapons/Flashbang/Audio/Flashbang_Cue.Flashbang_Cue" _returnvalue_2 (struct) 1.0 1.0 0.0 "/Game/VR_Weapons/Flashbang/Audio/FlashbangAttenuation.FlashbangAttenuation" null self)
                    (bind _returnvalue_6 (`GameplayStatics.SpawnEmitterAtLocation` "/Game/VR_Weapons/Flashbang/Particles/P_FlashBang.P_FlashBang" _returnvalue_2))
                    (set `self.Particle effect` _returnvalue_6)
                    (bind _returnvalue_7 (`AddComponent|NODE_AddPointLightComponent-0` :`bManualAttachment` true :`RelativeTransform` (`self.GetTransform`)))
                    (`|ExecutionSequence`
                      (:`then_0`
                        (bind _outhit_3 (`KismetSystemLibrary.LineTraceSingleForObjects` :`Start` _returnvalue :`End` (- _returnvalue (0.0 0.0 50.0)) :`ObjectTypes` (`|MakeArray` "ObjectTypeQuery1" :!type "EObjectTypeQuery Enum") :`DrawDebugType` (select `bool` (`self.Debug mode`) :`true` "ForDuration" :!type "EDrawDebugTrace Enum")))
                        (bind (_bblockinghit _binitialoverlap _time _distance _location _impactpoint _normal) (`GameplayStatics.BreakHitResult` _outhit_3))
                        (if _bblockinghit
                          (bind _oculus_quest_2 (`/Game/VR_Weapons/Global/Blueprints/GlobalFunctions.CheckDevice`))
                          (if _oculus_quest_2
                            (`GameplayStatics.SpawnEmitterAtLocation` "/Game/VR_Weapons/Flashbang/Particles/P_Flashbang_explosion_mark.P_FlashBang_explosion_mark" _location)
                            (else
                              (bind (_returnvalue_roll _returnvalue_pitch) (`KismetMathLibrary.BreakRotator` (`KismetMathLibrary.Conv_VectorToRotator` _normal)))
                              (bind _returnvalue_8 (`GameplayStatics.SpawnDecalAtLocation` "/Game/VR_Weapons/Flashbang/Materials/M_Flashbang_explosion_decal.M_Flashbang_explosion_decal" (* (`KismetMathLibrary.MakeVector` 1.0 135.0 135.0) (`KismetMathLibrary.RandomFloatInRange` 0.4 0.8)) _location (`KismetMathLibrary.MakeRotator` _returnvalue_roll _returnvalue_pitch (`KismetMathLibrary.RandomFloatInRange` 0.0 360.0)) 25.0))
                              (`DecalComponent.SetFadeScreenSize` _returnvalue_8 0.01) ; how small on the screen before fading out
                              (`DecalComponent.SetFadeOut` _returnvalue_8 15.0 20.0 false))))
                        (`RadialForceComponent.FireImpulse` (`self.RadialForce`))
                        (`PrimitiveComponent.AddAngularImpulseInDegrees` _flashbang_grenade (`KismetMathLibrary.MakeVector` (`KismetMathLibrary.RandomFloatInRange` 0.0 400.0) (`KismetMathLibrary.RandomFloatInRange` 0.0 400.0) (`KismetMathLibrary.RandomFloatInRange` 0.0 400.0)) "None" true)
                        (`PrimitiveComponent.AddImpulse` _flashbang_grenade (0.0 0.0 200.0) "None" false)
                        (if (or (`self.Flashbang heard`) (`self.Close interior proximity`))
                          (`KismetSystemLibrary.Delay` 0.1)
                          (bind _returnvalue_9 (`GameplayStatics.CreateSound2D` "/Game/VR_Weapons/Flashbang/Audio/Ear_ringing.Ear_ringing" 1.0 1.0 0.0 null)) ; add ear ringing sound effect
                          (`AudioComponent.FadeIn` _returnvalue_9 2.5 1.0 0.0 "Linear")
                          (`GameplayStatics.PushSoundMixModifier` "/Game/VR_Weapons/Flashbang/Audio/FlashbangSoundMix.FlashbangSoundMix") ; To simulate deafness the sound mix modifier.is applied.\nThis will muffle all sounds that belong to the default "Master"\nsound class\n\nAll sounds belong to the Master class by default, if you \ndon't want the flashbang to muffle a sound effect \n(such as a UI sound) please create and apply a new sound \nclass to that sound effect or use the "weapons sounds"\nclass which will only muffle the sound slightly.
                          (`KismetSystemLibrary.Delay` (`KismetMathLibrary.MapRangeClamped` (`self.explosion distance`) 0.3 1.0 (`self.Stun duration min`) (`self.Stun duration max`)))
                          (`GameplayStatics.PopSoundMixModifier` "/Game/VR_Weapons/Flashbang/Audio/FlashbangSoundMix.FlashbangSoundMix") ; fade out sound mix modifier\ndefault fade time is set to 5 seconds
                          (`AudioComponent.FadeOut` _returnvalue_9 10.0 0.0 "Linear") ; fade out ear ringing sound effect
                        ))
                      (:`then_1`
                        (`KismetSystemLibrary.Delay` 0.1)
                        (`ActorComponent.K2_DestroyComponent` _returnvalue_7)
                        (set `ParticleSystemComponent.bOverrideLODMethod` true _particle_effect)
                        (set `ParticleSystemComponent.LODMethod` "PARTICLESYSTEMLODMETHOD_DirectSet" _particle_effect) ; stop LOD changing after explosion
                      )))))))
          (:`then_2`
            ;[0 0 0] Stop simulating physics after a few seconds
            (`KismetSystemLibrary.Delay` 10.0)
            (for _array_element_2 (`|MakeArray` (`self.Lever`) (`/Game/VR_Weapons/Flashbang/Blueprints/BP_Pin.Pin` (`self.BP_pin`)) (`self.Flashbang_grenade`))
              (`/Engine/EditorBlueprintResources/StandardMacros.IsValid` _array_element_2
                (:`Is Valid`
                  (`PrimitiveComponent.SetSimulatePhysics` _array_element_2 false))))))))))

(event `Hit`
  (params (HitComponent :type "PrimitiveComponent Object Reference") (OtherActor :type "Actor Object Reference") (OtherComp :type "PrimitiveComponent Object Reference") (NormalImpulse :type "Vector Structure") (Hit :type "HitResult Structure (by ref)"))
  ;[0 0 0] Release
  (`/Engine/EditorBlueprintResources/StandardMacros.DoOnce` false
    (:`Completed`
      (`KismetSystemLibrary.PrintString` "Hit" true true (struct :`R` 0.897669 :`G` 1.0 :`A` 1.0))
      (`GameplayStatics.PlaySoundAtLocation` "/Game/VR_Weapons/Flashbang/Audio/Flashbang_lever_impact_Cue.Flashbang_lever_impact_Cue" (`.Location` (`GameplayStatics.BreakHitResult` Hit)) (struct) 1.0 1.0 0.0 "/Game/VR_Weapons/Global/Audio/Small_object_Attenuation.Small_object_Attenuation" null null))))

(event `/Game/VR_Weapons/Pawn/Blueprints/PickupActorInterface.Drop`
  (bind _debug_mode (`self.Debug mode`))
  (bind _debug_mode_2 (`self.Debug mode`))
  ;[0 0 0] Release
  (`PrimitiveComponent.SetSimulatePhysics` (`self.Flashbang_grenade`) true)
  (`self.K2_DetachFromActor` "KeepWorld" "KeepWorld" "KeepWorld")
  (set `self.Grabbed` false)
  (`PlayerController.StopHapticEffect` (`GameplayStatics.GetPlayerController` 0) (`self.Hand`))
  (set `self.MotionController` null) ; clear reference
  (`KismetSystemLibrary.PrintString` "Flashbang dropped" _debug_mode _debug_mode (struct :`R` 0.728 :`G` 0.364 :`B` 0.003 :`A` 1.0))
  (if (`self.pin removed`)
    (`|ExecutionSequence`
      (:`then_0`
        (goto _label))
      (:`then_1`
        _))
    (else
      (set `PrimitiveComponent.bGenerateOverlapEvents` true (`self.Flashbang_grenade`))))
  (`self.Pin overlap events` false)
  (`KismetSystemLibrary.PrintString` "Collision reset for flashbang & pin" _debug_mode_2 _debug_mode_2 (struct :`R` 0.159453 :`G` 1.0 :`A` 1.0)))

(event `self.Flashbang_grenade.OnComponentHit`
  (params (HitComponent :type "PrimitiveComponent Object Reference") (OtherActor :type "Actor Object Reference") (OtherComp :type "PrimitiveComponent Object Reference") (NormalImpulse :type "Vector Structure") (Hit :type "HitResult Structure (by ref)"))
  (bind _returnvalue (`KismetMathLibrary.VSize` NormalImpulse))
  ;[0 0 0] Impact sound
  (`GameplayStatics.PlaySoundAtLocation` "/Game/VR_Weapons/Flashbang/Audio/Flashbang_impact_Cue.Flashbang_impact_Cue" (`.Location` (`GameplayStatics.BreakHitResult` Hit)) (struct) (`KismetMathLibrary.MapRangeClamped` _returnvalue 20.0 120.0 0.0 1.0) (`KismetMathLibrary.MapRangeClamped` _returnvalue 0.0 50.0 0.7 1.0) 0.0 "/Game/VR_Weapons/Global/Audio/Small_object_Attenuation.Small_object_Attenuation" "/Game/VR_Weapons/Flashbang/Audio/FlashBangConcurrency.FlashBangConcurrency" null))

(fn `Bounce line traces inside`
  (params (`Target point` :type "Vector Structure") (`Target Actor` :type "Object Object Reference"))
  (returns (`Line trace hit actor` :type Boolean))
  (locals (`Random initial target` :type "Vector Structure" :default (0.0 0.0 0.0)) (Target_point :type "Vector Structure" :default (0.0 0.0 0.0)) (Target_actor :type "Object Object Reference"))
  (bind _returnvalue (`self.K2_GetActorLocation`))
  (bind _returnvalue_2 (+ _returnvalue (`local.Random initial target`)))
  (set `local.Target_point` `Target point`)
  ;[0 0 0] Bounce 1
  (set `local.Target_actor` `Target Actor`)
  (set `local.Random initial target` (`KismetMathLibrary.MakeVector` (`KismetMathLibrary.RandomFloatInRange` -500.0 500.0) (`KismetMathLibrary.RandomFloatInRange` -500.0 500.0) 750.0))
  (bind (_outhit _returnvalue_3) (`KismetSystemLibrary.LineTraceSingle` :`Start` (+ _returnvalue (0.0 0.0 10.0)) :`End` _returnvalue_2 :`TraceChannel` (`self.Trace channel`) :`DrawDebugType` (select `bool` (`self.Debug mode`) :`true` "ForDuration" :!type "EDrawDebugTrace Enum") :`TraceColor` (struct :`R` 0.933729 :`G` 0.230999 :`B` 1.0 :`A` 1.0))) ; Bounce 1
  (if _returnvalue_3
    (bind (_bblockinghit _binitialoverlap _time _distance _location _impactpoint _normal _impactnormal) (`GameplayStatics.BreakHitResult` _outhit))
    ;[0 0 0] Bounce 2
    (bind _outhit_2 (`KismetSystemLibrary.LineTraceSingle` :`Start` (+ _location (* _impactnormal 10.0)) :`End` (`KismetMathLibrary.MirrorVectorByNormal` _returnvalue_2 _impactnormal) :`TraceChannel` (`self.Trace channel`) :`DrawDebugType` (select `bool` (`self.Debug mode`) :`true` "ForDuration" :!type "EDrawDebugTrace Enum") :`TraceColor` (struct :`R` 0.238443 :`G` 0.492216 :`B` 1.0 :`A` 1.0))) ; Bounce 2
    (bind (_bblockinghit_2 _binitialoverlap_2 _time_2 _distance_2 _location_2 _impactpoint_2 _normal_2 _impactnormal_2) (`GameplayStatics.BreakHitResult` _outhit_2))
    ;[0 0 0] Try to reach player
    (bind _outhit_3 (`KismetSystemLibrary.LineTraceSingle` :`Start` (+ _impactpoint_2 (* _impactnormal_2 10.0)) :`End` (`local.Target_point`) :`TraceChannel` (`self.Trace channel`) :`DrawDebugType` (select `bool` (`self.Debug mode`) :`true` "ForDuration" :!type "EDrawDebugTrace Enum") :`TraceColor` (struct :`R` 1.0 :`G` 0.417922 :`B` 0.237019 :`A` 1.0))) ; Try to reach player
    (return (== (`.HitActor` (`GameplayStatics.BreakHitResult` _outhit_3)) (`local.Target_actor`)))))

(fn `explosion distance`
  (returns (ReturnValue :type "Float (double-precision)"))
  (locals (`min brightness` :type "Float (double-precision)" :default 0.3) (`max brightness` :type "Float (double-precision)" :default 1.0))
  (bind _blast_radius (`self.blast radius`))
  (return (`KismetMathLibrary.MapRangeClamped` (`KismetMathLibrary.Vector_Distance` (`SceneComponent.K2_GetComponentLocation` (`self.Player head`)) (`self.K2_GetActorLocation`)) (/ _blast_radius 2.0) _blast_radius (`local.max brightness`) (`local.min brightness`))))

(fn `GripHandGuard`
  (params (Hand :type "/Game/VR_Weapons/Pawn/Blueprints/BP_MotionController Object Reference"))
  (returns (HandguardGrabbed :type Boolean))
  (return false))

(fn `InsertMagazine`
  (params (OverlappedComponent :type "PrimitiveComponent Object Reference") (WeaponType :type "/Game/VR_Weapons/Pawn/Blueprints/E_WeaponType Enum" :default "NewEnumerator0"))
  (returns (`Magazine Compatible` :type Boolean) (`Weapon Mesh` :type "StaticMeshComponent Object Reference") (`Weapon Actor` :type "/Game/VR_Weapons/Global/Blueprints/BP_Gun Object Reference"))
  (return false null null))

(fn `Lever Pressure Haptics`
  (`/Game/VR_Weapons/Pawn/Blueprints/BP_MotionController.RumbleController` (`self.MotionController`) "/Game/VR_Weapons/Pawn/Haptics/Haptics_auto_firing.Haptics_auto_firing" 0.15 true))

(fn `LineTraceEnvironment`
  (params (`Line trace end` :type "Vector Structure"))
  (returns (Hit :type Boolean))
  (bind _returnvalue (`self.K2_GetActorLocation`))
  (bind (_outhit _returnvalue_2) (`KismetSystemLibrary.LineTraceSingle` (+ _returnvalue (0.0 0.0 10.0)) (+ _returnvalue `Line trace end`) (`self.Trace channel`)))
  (if _returnvalue_2
    (bind (_bblockinghit _binitialoverlap _time _distance _location _impactpoint _normal _impactnormal _physmat _hitactor) (`GameplayStatics.BreakHitResult` _outhit))
    (`KismetSystemLibrary.PrintString` (`KismetSystemLibrary.GetDisplayName` _hitactor) false false (struct :`R` 0.55183 :`G` 0.323558 :`B` 1.0 :`A` 1.0) 1.0)
    (return _bblockinghit)))

(fn `Pickup`
  (params (Hand :type "EControllerHand Enum" :default "Left") (`Grip or grab` :type "/Game/VR_Weapons/Pawn/Blueprints/E_GrabType Enum" :default "NewEnumerator1") (Actor :type "/Game/VR_Weapons/Pawn/Blueprints/BP_MotionController Object Reference") (AttachTo :type "SceneComponent Object Reference"))
  (returns (WeaponType :type "/Game/VR_Weapons/Pawn/Blueprints/E_WeaponType Enum") (GunGrabbed :type Boolean))
  (bind _returnvalue (`self.K2_GetRootComponent`))
  (bind _flashbang_grenade (`self.Flashbang_grenade`))
  (bind _debug_mode (`self.Debug mode`))
  (switch `/Game/VR_Weapons/Pawn/Blueprints/E_GrabType` `Grip or grab`
    (:`NewEnumerator1`
      (if (and (not (`self.Grabbed`)) (not (`self.pin removed`)))
        (set `self.MotionController` Actor)
        (set `self.Hand` Hand)
        (`PrimitiveComponent.SetSimulatePhysics` (`self.Flashbang_grenade`) false)
        (`SceneComponent.SetWorldScale3D` _returnvalue (`KismetMathLibrary.SelectVector` (1.0 -1.0 -1.0) (1.0 1.0 1.0) (`|EnumEquality` (`self.Hand`) "Left"))) ; Flip BP_flashbang if left hand grabbing
        (`SceneComponent.K2_AttachToComponent` _returnvalue AttachTo "FlashbangGripSocket" "SnapToTarget" "SnapToTarget" "KeepWorld" true)
        (`self.SetActorEnableCollision` (`self.BP_pin`) true) ; allow pin to be removed once flashbang has been picked up
        (`self.Pin overlap events` true)
        (set `PrimitiveComponent.bGenerateOverlapEvents` false _flashbang_grenade)
        (`PrimitiveComponent.SetCollisionEnabled` _flashbang_grenade "PhysicsOnly")
        (set `self.Grabbed` true)
        (return "NewEnumerator2" false)
        (else
          (`KismetSystemLibrary.PrintString` "Already grabbed or pin removed" _debug_mode _debug_mode (struct :`R` 1.0 :`A` 1.0)))))
    (:`NewEnumerator0`
      (`KismetSystemLibrary.PrintString` "Gripping instead of grabbing" _debug_mode _debug_mode (struct :`R` 1.0 :`A` 1.0)))))

(fn `Pin overlap events`
  (params (bGenerateOverlapEvents :type Boolean))
  (bind _bp_pin (`self.BP_pin`))
  (set `PrimitiveComponent.bGenerateOverlapEvents` bGenerateOverlapEvents (`/Game/VR_Weapons/Flashbang/Blueprints/BP_Pin.Pin` _bp_pin)) ; stop user from grabbing the pin once its removed
  (set `PrimitiveComponent.bGenerateOverlapEvents` bGenerateOverlapEvents (`/Game/VR_Weapons/Flashbang/Blueprints/BP_Pin.Pullring` _bp_pin)) ; stop user from grabbing the pullring once its removed
  (set `PrimitiveComponent.bGenerateOverlapEvents` bGenerateOverlapEvents (`/Game/VR_Weapons/Flashbang/Blueprints/BP_Pin.Overlap` _bp_pin)) ; Stop user from grabbing overlap collision box
)

(fn `PullTrigger`
  (returns (Fired :type Boolean))
  (return false))

(fn `Try to reach AI`
  (returns (`Actor hit` :type Boolean))
  (locals (`hit actor` :type Boolean :default false))
  (bind _enemy_character (`self.Enemy character`))
  (for _ (range (`self.Close proximity bounces`))
    (bind _line_trace_hit_actor (`self.Bounce line traces inside` (`SceneComponent.GetSocketLocation` (`Character.Mesh` _enemy_character) "Head") _enemy_character)) ; Bounce line traces off walls/objects in an attempt to reach actor
    (set `local.hit actor` _line_trace_hit_actor))
  (return (`local.hit actor`)))

(fn `UserConstructionScript`
  (`SphereComponent.SetSphereRadius` (`self.Player collision sphere`) (`self.blast radius`) true))