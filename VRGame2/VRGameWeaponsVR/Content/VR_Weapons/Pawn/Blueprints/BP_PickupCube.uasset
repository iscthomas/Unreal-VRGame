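; BP_PickupCube is a physics cube that can be picked up and dropped by a hand in the VR weapons setup.
; Pickup turns off physics and snaps the cube to the FlashbangGripSocket on the supplied component, keeping world scale.
; Drop re-enables physics and detaches it in place.
; Weapon-style functions for trigger, handguard and magazine are stubs returning false, and Pickup reports no gun grabbed.
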(event `Pickup_Event`
  (params (AttachTo :type "SceneComponent Object Reference") (Hand :type "EControllerHand Enum" :default "Left"))
  (`PrimitiveComponent.SetSimulatePhysics` (`self.StaticMeshComponent`) false)
  (`SceneComponent.K2_AttachToComponent` (`self.K2_GetRootComponent`) AttachTo "FlashbangGripSocket" "SnapToTarget" "SnapToTarget" "KeepWorld" false))

(event `/Game/VR_Weapons/Pawn/Blueprints/PickupActorInterface.Drop`
  (`PrimitiveComponent.SetSimulatePhysics` (`self.StaticMeshComponent`) true)
  (`self.K2_DetachFromActor` "KeepWorld" "KeepWorld" "KeepWorld"))

(fn `GrabHandGuard`
  (params (Hand :type "/Game/VR_Weapons/Pawn/Blueprints/BP_MotionController Object Reference"))
  (returns (HandguardGrabbed :type Boolean))
  (return false))

(fn `InsertMagazine`
  (params (OverlappedComponent :type "PrimitiveComponent Object Reference") (WeaponType :type "/Game/VR_Weapons/Pawn/Blueprints/E_WeaponType Enum" :default "NewEnumerator0"))
  (returns (`Magazine Compatible` :type Boolean) (`Weapon Mesh` :type "StaticMeshComponent Object Reference") (`Weapon Actor` :type "/Game/VR_Weapons/Global/Blueprints/BP_Gun Object Reference"))
  (return false null null))

(fn `Pickup`
  (params (Hand :type "EControllerHand Enum" :default "Left") (`Grip or grab` :type "/Game/VR_Weapons/Pawn/Blueprints/E_GrabType Enum" :default "NewEnumerator1") (Actor :type "/Game/VR_Weapons/Pawn/Blueprints/BP_MotionController Object Reference") (AttachTo :type "SceneComponent Object Reference"))
  (returns (WeaponType :type "/Game/VR_Weapons/Pawn/Blueprints/E_WeaponType Enum") (GunGrabbed :type Boolean))
  (`self.Pickup_Event` AttachTo Hand)
  (return "NewEnumerator0" false))

(fn `PullTrigger`
  (returns (Fired :type Boolean))
  (return false))

(fn `UserConstructionScript`)