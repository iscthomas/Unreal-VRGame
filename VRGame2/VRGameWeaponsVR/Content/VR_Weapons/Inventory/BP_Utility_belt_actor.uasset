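; BP_Utility_belt_actor is the VR utility belt inventory, storing weapons and flashbangs in six slots and magazines or shotgun cartridges in an ammo slot.
; AddItemToInventory snaps compatible overlapping items into slots, while slot overlaps drive scaling and controller haptics.
; Stored items appear when a motion controller nears and hide after a delay, with ammo filtered by WeaponTypeInHand.
; The construction script can swap to masked slot materials for Quest performance.
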(event `self.Slot1.OnComponentBeginOverlap`
  (params (OverlappedComponent :type "PrimitiveComponent Object Reference") (OtherActor :type "Actor Object Reference") (OtherComp :type "PrimitiveComponent Object Reference") (OtherBodyIndex :type Integer) (bFromSweep :type Boolean) (SweepResult :type "HitResult Structure (by ref)"))
  ;[0 0 0] Weapons slot overlap begin
  (`self.Overlap begin` OverlappedComponent (`self.Overlapped scale`) OtherActor))

(event `self.Slot2.OnComponentBeginOverlap`
  (params (OverlappedComponent :type "PrimitiveComponent Object Reference") (OtherActor :type "Actor Object Reference") (OtherComp :type "PrimitiveComponent Object Reference") (OtherBodyIndex :type Integer) (bFromSweep :type Boolean) (SweepResult :type "HitResult Structure (by ref)"))
  ;[0 0 0] Weapons slot overlap begin
  (`self.Overlap begin` OverlappedComponent (`self.Overlapped scale`) OtherActor))

(event `self.Ammo slot.OnComponentBeginOverlap`
  (params (OverlappedComponent :type "PrimitiveComponent Object Reference") (OtherActor :type "Actor Object Reference") (OtherComp :type "PrimitiveComponent Object Reference") (OtherBodyIndex :type Integer) (bFromSweep :type Boolean) (SweepResult :type "HitResult Structure (by ref)"))
  (bind _returnvalue (`self.GetAttachParentActor` OtherActor))
  ;[0 0 0] Ammo slot overlap begin
  (if (`self.ActorHasTag` OtherActor "Mag")
    (`SceneComponent.SetRelativeScale3D` OverlappedComponent (0.5 0.5 0.5))
    (`/Engine/EditorBlueprintResources/StandardMacros.IsValid` _returnvalue
      (:`Is Valid`
        (bind _asbp_motion_controller (cast `/Game/VR_Weapons/Pawn/Blueprints/BP_MotionController` _returnvalue)
          (:`then`
            (`/Game/VR_Weapons/Pawn/Blueprints/BP_MotionController.RumbleController` _asbp_motion_controller "/Game/VR_Weapons/Pawn/Haptics/Haptics_single.Haptics_single" 0.3 false))
          (:`CastFailed`
            (bind _asbp_motion_controller_2 (cast `/Game/VR_Weapons/Pawn/Blueprints/BP_MotionController` (`self.GetAttachParentActor` _returnvalue)))
            (`/Game/VR_Weapons/Pawn/Blueprints/BP_MotionController.RumbleController` _asbp_motion_controller_2 "/Game/VR_Weapons/Pawn/Haptics/Haptics_single.Haptics_single" 0.3 false)))))))

(event `self.Slot3.OnComponentBeginOverlap`
  (params (OverlappedComponent :type "PrimitiveComponent Object Reference") (OtherActor :type "Actor Object Reference") (OtherComp :type "PrimitiveComponent Object Reference") (OtherBodyIndex :type Integer) (bFromSweep :type Boolean) (SweepResult :type "HitResult Structure (by ref)"))
  ;[0 0 0] Weapons slot overlap begin
  (`self.Overlap begin` OverlappedComponent (`self.Overlapped scale`) OtherActor))

(event `self.Slot4.OnComponentBeginOverlap`
  (params (OverlappedComponent :type "PrimitiveComponent Object Reference") (OtherActor :type "Actor Object Reference") (OtherComp :type "PrimitiveComponent Object Reference") (OtherBodyIndex :type Integer) (bFromSweep :type Boolean) (SweepResult :type "HitResult Structure (by ref)"))
  ;[0 0 0] Weapons slot overlap begin
  (`self.Overlap begin` OverlappedComponent (`self.Overlapped scale`) OtherActor))

(event `self.Slot5.OnComponentBeginOverlap`
  (params (OverlappedComponent :type "PrimitiveComponent Object Reference") (OtherActor :type "Actor Object Reference") (OtherComp :type "PrimitiveComponent Object Reference") (OtherBodyIndex :type Integer) (bFromSweep :type Boolean) (SweepResult :type "HitResult Structure (by ref)"))
  ;[0 0 0] Weapons slot overlap begin
  (`self.Overlap begin` OverlappedComponent (`self.Overlapped scale`) OtherActor))

(event `self.Ammo slot.OnComponentEndOverlap`
  (params (OverlappedComponent :type "PrimitiveComponent Object Reference") (OtherActor :type "Actor Object Reference") (OtherComp :type "PrimitiveComponent Object Reference") (OtherBodyIndex :type Integer))
  ;[0 0 0] Ammo slot overlap end
  (`SceneComponent.SetRelativeScale3D` OverlappedComponent (0.4 0.4 0.4)))

(event `self.Slot 6.OnComponentBeginOverlap`
  (params (OverlappedComponent :type "PrimitiveComponent Object Reference") (OtherActor :type "Actor Object Reference") (OtherComp :type "PrimitiveComponent Object Reference") (OtherBodyIndex :type Integer) (bFromSweep :type Boolean) (SweepResult :type "HitResult Structure (by ref)"))
  ;[0 0 0] Weapons slot overlap begin
  (`self.Overlap begin` OverlappedComponent (`self.Overlapped scale`) OtherActor))

(event `Update Utility belt`
  (params (`Weapon type` :type "/Game/VR_Weapons/Pawn/Blueprints/E_WeaponType Enum" :default "NewEnumerator0"))
  ;[0 0 0] Update visibility of ammo depending on the weapon picked up (called from BP_motioncontroller)
  (set `self.Weapon type in hand` `Weapon type`)
  (for _array_element (`self.GetAttachedActors` true)
    (`self.Update ammo visibility & collision` _array_element)))

(event `self.Slot1.OnComponentEndOverlap`
  (params (OverlappedComponent :type "PrimitiveComponent Object Reference") (OtherActor :type "Actor Object Reference") (OtherComp :type "PrimitiveComponent Object Reference") (OtherBodyIndex :type Integer))
  ;[0 0 0] Weapons slot overlap end
  (`self.Overlap end delayed` OverlappedComponent (`self.Default scale`)))

(event `Hand empty`
  ;[0 0 0] Change weapon type to None when a gun is droppped (called from BP_motioncontroller)
  (set `self.Weapon type in hand` "NewEnumerator0"))

(event `self.Slot2.OnComponentEndOverlap`
  (params (OverlappedComponent :type "PrimitiveComponent Object Reference") (OtherActor :type "Actor Object Reference") (OtherComp :type "PrimitiveComponent Object Reference") (OtherBodyIndex :type Integer))
  ;[0 0 0] Weapons slot overlap end
  (`self.Overlap end delayed` OverlappedComponent (`self.Default scale`)))

(event `self.Slot3.OnComponentEndOverlap`
  (params (OverlappedComponent :type "PrimitiveComponent Object Reference") (OtherActor :type "Actor Object Reference") (OtherComp :type "PrimitiveComponent Object Reference") (OtherBodyIndex :type Integer))
  ;[0 0 0] Weapons slot overlap end
  (`self.Overlap end delayed` OverlappedComponent (`self.Default scale`)))

(event `Item added`
  (params (Slot :type "SceneComponent Object Reference") (NewScale3D :type "Vector Structure"))
  (`self.Overlap end delayed` Slot NewScale3D))

(event `self.Slot4.OnComponentEndOverlap`
  (params (OverlappedComponent :type "PrimitiveComponent Object Reference") (OtherActor :type "Actor Object Reference") (OtherComp :type "PrimitiveComponent Object Reference") (OtherBodyIndex :type Integer))
  ;[0 0 0] Weapons slot overlap end
  (`self.Overlap end delayed` OverlappedComponent (`self.Default scale`)))

(event `self.Slot5.OnComponentEndOverlap`
  (params (OverlappedComponent :type "PrimitiveComponent Object Reference") (OtherActor :type "Actor Object Reference") (OtherComp :type "PrimitiveComponent Object Reference") (OtherBodyIndex :type Integer))
  ;[0 0 0] Weapons slot overlap end
  (`self.Overlap end delayed` OverlappedComponent (`self.Default scale`)))

(event `self.Slot 6.OnComponentEndOverlap`
  (params (OverlappedComponent :type "PrimitiveComponent Object Reference") (OtherActor :type "Actor Object Reference") (OtherComp :type "PrimitiveComponent Object Reference") (OtherBodyIndex :type Integer))
  ;[0 0 0] Weapons slot overlap end
  (`self.Overlap end delayed` OverlappedComponent (`self.Default scale`)))

(event `self.Utility belt collision.OnComponentBeginOverlap`
  (params (OverlappedComponent :type "PrimitiveComponent Object Reference") (OtherActor :type "Actor Object Reference") (OtherComp :type "PrimitiveComponent Object Reference") (OtherBodyIndex :type Integer) (bFromSweep :type Boolean) (SweepResult :type "HitResult Structure (by ref)"))
  ;[0 0 0] Toggle utility belt visibility/collision when overlapping with motion controller
  (cast `/Game/VR_Weapons/Pawn/Blueprints/BP_MotionController` OtherActor)
  (`self.Toggle attached actors visibility/collision` false)
  (`self.Update Utility belt` (`self.Weapon type in hand`))
  (set `self.Overlapped` true))

(event `self.Utility belt collision.OnComponentEndOverlap`
  (params (OverlappedComponent :type "PrimitiveComponent Object Reference") (OtherActor :type "Actor Object Reference") (OtherComp :type "PrimitiveComponent Object Reference") (OtherBodyIndex :type Integer))
  ;[0 0 0] Toggle utility belt visibility/collision when overlapping with motion controller
  (cast `/Game/VR_Weapons/Pawn/Blueprints/BP_MotionController` OtherActor)
  (set `self.Overlapped` false)
  (`KismetSystemLibrary.Delay` 0.4)
  (if (and (not (`self.Overlapped`)) (< (`KismetArrayLibrary.Array_Length` (`PrimitiveComponent.GetOverlappingActors` OverlappedComponent "/Game/VR_Weapons/Pawn/Blueprints/BP_MotionController.BP_MotionController_C")) 1))
    (`self.Toggle attached actors visibility/collision` true)))

(fn `Add item to inventory`
  (params (Item :type "Actor Object Reference"))
  (returns (Added :type Boolean))
  (locals (`Overlapped slot` :type "StaticMeshComponent Object Reference") (`Parent actor` :type "Actor Object Reference"))
  (bind _item (`local.Item`))
  (bind _item_2 (`local.Item`))
  (`/Engine/EditorBlueprintResources/StandardMacros.IsValid` Item
    (:`Is Valid`
      (for _array_element (`self.Slots`)
        (bind _output_get (set `local.Overlapped slot` _array_element))
        (bind _returnvalue (`self.Is slot compatible` _output_get (`local.Item`)))
        (if _returnvalue
          (set `local.Parent actor` (`self.GetAttachParentActor` (`local.Item`))) ; get motion controller reference
          (message `/Game/VR_Weapons/Pawn/Blueprints/PickupActorInterface.Drop` _item) ; call drop event to clear motion controller variables in BP_gun
          (bind _asbp_gun (cast `/Game/VR_Weapons/Global/Blueprints/BP_Gun` _item)
            (:`then`
              (set `/Game/VR_Weapons/Global/Blueprints/BP_Gun.Weapon stored in utility belt` true _asbp_gun))
            (:`CastFailed`
              _))
          (`self.Rumble motion controller` (`local.Parent actor`))
          (`|ExecutionSequence`
            (:`then_0`
              (`self.K2_AttachToComponent` (`local.Item`) (`local.Overlapped slot`) "None" "SnapToTarget" "SnapToTarget" "SnapToTarget" true)
              (`self.Item added` (`local.Overlapped slot`) (`KismetMathLibrary.SelectVector` (0.4 0.4 0.4) (`self.Default scale`) (== (`local.Overlapped slot`) (`self.Ammo slot`))))
              (return _returnvalue))
            (:`then_1`
              (if (not (and (`|EnumEquality` (`self.Weapon type in hand`) "NewEnumerator0") (`self.ActorHasTag` (`local.Item`) "Mag")))
                (`self.Update ammo visibility & collision` _item_2) ; hide magazine if it doesn't match current weapon in hand
                (else
                  ;[0 0 0] Cast to magazine & shotgun cartridge cartridge to set the weapon in type in hand
                  (bind _asbp_magazine (cast `/Game/VR_Weapons/Global/Blueprints/BP_Magazine` _item_2)
                    (:`then`
                      (set `self.Weapon type in hand` (`/Game/VR_Weapons/Global/Blueprints/BP_Magazine.MagazineType` _asbp_magazine)))
                    (:`CastFailed`
                      (cast `/Game/VR_Weapons/Guns/Shotgun/Blueprints/BP_Shotgun_cartridge` _item_2)
                      (set `self.Weapon type in hand` "NewEnumerator6")))
                  (for _array_element_2 (`self.GetAttachedActors` true)
                    (`self.Update ammo visibility & collision` _array_element_2) ; Show ammo type added and hide all over types
                  ))))))))))

(fn `Add magazine to inventory`
  (params (Magazine :type "/Game/VR_Weapons/Global/Blueprints/BP_Magazine Object Reference") (Bullets :type Integer))
  (returns (Added :type Boolean))
  (return false))

(fn `Is slot compatible`
  (params (`Overlapped Slot` :type "StaticMeshComponent Object Reference") (Item :type "Actor Object Reference"))
  (returns (ReturnValue :type Boolean))
  (locals (`Flashbang compatible` :type Boolean))
  (bind _overlapped_slot (`local.Overlapped slot`))
  (bind _overlapped_slot_2 (`local.Overlapped slot`))
  (bind _ammo_slot (`self.Ammo slot`))
  (bind _item (`local.Item`))
  (bind _returnvalue (!= _overlapped_slot _ammo_slot))
  ;[0.728 0.364 0.003] Flashbang
  (bind _asbp_flashbang (cast `/Game/VR_Weapons/Flashbang/Blueprints/BP_Flashbang` Item)
    (:`then`
      (if (> (`SceneComponent.GetNumChildrenComponents` _overlapped_slot_2) 1)
        (bind _returnvalue_2 (not (`/Game/VR_Weapons/Flashbang/Blueprints/BP_Flashbang.pin removed` _asbp_flashbang)))
        (set `local.Flashbang compatible` (and _returnvalue_2 (or (== (`SceneComponent.GetChildComponent` _overlapped_slot_2 1) null) (`self.ActorHasTag` (`ActorComponent.GetOwner` (`SceneComponent.GetChildComponent` _overlapped_slot_2 1)) "Flashbang"))))
        (else
          (set `local.Flashbang compatible` _returnvalue_2))))
    (:`CastFailed`
      _))
  (return (and (or (`PrimitiveComponent.IsOverlappingActor` _overlapped_slot (`|GetArrayItem` (`self.GetAttachedActors` _item true))) (`PrimitiveComponent.IsOverlappingActor` _overlapped_slot _item)) (or (and (!= (`SceneComponent.GetNumChildrenComponents` _overlapped_slot) 2) (`self.ActorHasTag` (`local.Item`) "Weapon") _returnvalue) (and (== _overlapped_slot _ammo_slot) (`self.ActorHasTag` (`local.Item`) "Mag")) (and _returnvalue (`local.Flashbang compatible`))))))

(fn `Overlap begin`
  (params (Slot :type "SceneComponent Object Reference") (NewScale3D :type "Vector Structure") (Weapon :type "Actor Object Reference"))
  (bind _returnvalue (`self.GetAttachParentActor` Weapon))
  (bind _slot (`local.Slot`))
  (bind _returnvalue_2 (`self.GetAttachParentActor` (`local.Weapon`)))
  (bind _returnvalue_3 (`self.GetAttachParentActor` _returnvalue_2))
  (`/Engine/EditorBlueprintResources/StandardMacros.IsValid` _returnvalue
    (:`Is Valid`
      (if (not (and (`self.ActorHasTag` Weapon "Mag") (not (`self.ActorHasTag` _returnvalue "Weapon"))))
        (if (not (< (`SceneComponent.GetNumChildrenComponents` _slot) 2)) :!label _label
          ;[0 0 0] allow overlap if flashbang overlaps slot that already contains a flashbang
          (cast `/Game/VR_Weapons/Flashbang/Blueprints/BP_Flashbang` (`ActorComponent.GetOwner` (`SceneComponent.GetChildComponent` _slot 1))) ; Is flashbang
          (cast `/Game/VR_Weapons/Flashbang/Blueprints/BP_Flashbang` (`local.Weapon`)))
        (`SceneComponent.SetRelativeScale3D` (`local.Slot`) (`local.NewScale3D`))
        (`self.Toggle attached actors visibility/collision` false)
        (`self.Update Utility belt` (`self.Weapon type in hand`))
        ;[0 0 0] try to get parent actor (motion controller) to apply vibration
        (`/Engine/EditorBlueprintResources/StandardMacros.IsValid` _returnvalue_2
          (:`Is Valid`
            (bind _asbp_motion_controller (cast `/Game/VR_Weapons/Pawn/Blueprints/BP_MotionController` _returnvalue_2)
              (:`then`
                (`/Game/VR_Weapons/Pawn/Blueprints/BP_MotionController.RumbleController` _asbp_motion_controller "/Game/VR_Weapons/Pawn/Haptics/Haptics_single.Haptics_single" 0.3 false))
              (:`CastFailed`
                (`/Engine/EditorBlueprintResources/StandardMacros.IsValid` _returnvalue_3
                  (:`Is Valid`
                    (bind _asbp_motion_controller_2 (cast `/Game/VR_Weapons/Pawn/Blueprints/BP_MotionController` _returnvalue_3))
                    (`/Game/VR_Weapons/Pawn/Blueprints/BP_MotionController.RumbleController` _asbp_motion_controller_2 "/Game/VR_Weapons/Pawn/Haptics/Haptics_single.Haptics_single" 0.3 false)))))))))
    (:`Is Not Valid`
      (goto _label))))

(fn `Overlap end`
  (params (Target :type "PrimitiveComponent Object Reference") (NewScale3D :type "Vector Structure"))
  (`SceneComponent.SetRelativeScale3D` Target NewScale3D)
  (if (< (`KismetArrayLibrary.Array_Length` (`PrimitiveComponent.GetOverlappingActors` (`self.Utility belt collision`) "/Game/VR_Weapons/Pawn/Blueprints/BP_MotionController.BP_MotionController_C")) 1)
    (`self.Toggle attached actors visibility/collision` true)))

(fn `Rumble motion controller`
  (params (MotionController :type "Actor Object Reference"))
  (bind _asbp_motion_controller (cast `/Game/VR_Weapons/Pawn/Blueprints/BP_MotionController` MotionController)
    (:`then`
      (`/Game/VR_Weapons/Pawn/Blueprints/BP_MotionController.RumbleController` _asbp_motion_controller "/Game/VR_Weapons/Pawn/Haptics/Haptics_single.Haptics_single" 0.5 false)
      (`KismetSystemLibrary.PrintString` "Cast sucessful" true true (struct :`R` 0.220479 :`G` 1.0 :`A` 1.0) 5.0))
    (:`CastFailed`
      (`KismetSystemLibrary.PrintString` "Cast failed" true true (struct :`R` 1.0 :`G` 0.006678 :`A` 1.0) 5.0))))

(fn `Toggle attached actors visibility/collision`
  (params (`Hide actors` :type Boolean))
  (bind _hide_actors (`local.Hide actors`))
  (for _array_element (`self.Slots`)
    (for _array_element_2 (`SceneComponent.GetChildrenComponents` _array_element true)
      (bind _returnvalue (`ActorComponent.GetOwner` _array_element_2))
      (`self.SetActorHiddenInGame` _returnvalue _hide_actors) ; Show weapon actors
      (`self.SetActorEnableCollision` _returnvalue (not _hide_actors)) ; disable collision for all attached actors
      (`self.SetActorEnableCollision` true) ; enable utility belt collision
    )))

(fn `Update ammo visibility & collision`
  (params (`attached actor` :type "Actor Object Reference"))
  (bind _attached_actor (`local.attached actor`))
  (bind _attached_actor_2 (`local.attached actor`))
  (bind _returnvalue (`|EnumEquality` "NewEnumerator6" (`self.Weapon type in hand`)))
  (bind _asbp_magazine (cast `/Game/VR_Weapons/Global/Blueprints/BP_Magazine` `attached actor`)
    (:`then`
      (bind _returnvalue_2 (`|EnumEquality` (`/Game/VR_Weapons/Global/Blueprints/BP_Magazine.MagazineType` _asbp_magazine) (`self.Weapon type in hand`)))
      (`self.SetActorEnableCollision` _attached_actor_2 _returnvalue_2)
      (`self.SetActorHiddenInGame` _attached_actor (not _returnvalue_2)))
    (:`CastFailed`
      (cast `/Game/VR_Weapons/Guns/Shotgun/Blueprints/BP_Shotgun_cartridge` `attached actor`)
      (`self.SetActorEnableCollision` _attached_actor_2 _returnvalue)
      (`self.SetActorHiddenInGame` _attached_actor (not _returnvalue)))))

(fn `UserConstructionScript`
  (locals (`Use masked material for Oculus Quest optimisation` :type Boolean :default false))
  (bind _output_get (set `self.Slots` (`|MakeArray` (`self.Slot1`) (`self.Slot2`) (`self.Slot3`) (`self.Slot4`) (`self.Slot5`) (`self.Ammo slot`) (`self.Slot 6`))))
  (bind _oculus_quest (`/Game/VR_Weapons/Global/Blueprints/GlobalFunctions.CheckDevice`))
  (if (and _oculus_quest (`local.Use masked material for Oculus Quest optimisation`))
    (for _array_element _output_get
      (`PrimitiveComponent.SetMaterial` _array_element 0 "/Game/VR_Weapons/Inventory/Materials/MI_UtitilyBeltSlot_masked.MI_UtitilyBeltSlot_masked") ; Optimise by switching to masked material instead of using transparent if on Quest
    )
    (bind _returnvalue (`PrimitiveComponent.CreateDynamicMaterialInstance` (`self.Ammo slot`) 0 "/Game/VR_Weapons/Inventory/Materials/MI_UtitilyBeltSlot_masked.MI_UtitilyBeltSlot_masked" "None"))
    (`MaterialInstanceDynamic.SetVectorParameterValue` _returnvalue "Colour2" (struct :`R` 0.184475 :`G` 0.473532 :`B` 1.0 :`A` 1.0))
    (else
      (bind _returnvalue_2 (`PrimitiveComponent.CreateDynamicMaterialInstance` (`self.Ammo slot`) 0 "/Game/VR_Weapons/Inventory/Materials/MI_UtitilyBeltSlot.MI_UtitilyBeltSlot" "None"))
      (`MaterialInstanceDynamic.SetVectorParameterValue` _returnvalue_2 "Colour2" (struct :`R` 0.184475 :`G` 0.473532 :`B` 1.0 :`A` 1.0)))))