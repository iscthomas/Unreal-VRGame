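; BP_Silencer is a grabbable VR weapon attachment that snaps onto a compatible BP_Gun.
; Overlapping the gun's tagged collision attaches it to the Silencer socket, provided weapon type matches, no silencer is fitted and automatic fire sound isn't playing.
; Pickup attaches it to a hand socket, sets the right-hand AnimBP grip, clears the gun's silencer flag and briefly blocks re-attachment.
; Dropping detaches it, enables physics and resets the grip.
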(event `self.ReceiveBeginPlay`
  (if (`self.Start Simulating Physics`)
    (`PrimitiveComponent.SetSimulatePhysics` (`self.Silencer`) true)))

(event `self.Collision.OnComponentBeginOverlap`
  (params (OverlappedComponent :type "PrimitiveComponent Object Reference") (OtherActor :type "Actor Object Reference") (OtherComp :type "PrimitiveComponent Object Reference") (OtherBodyIndex :type Integer) (bFromSweep :type Boolean) (SweepResult :type "HitResult Structure (by ref)"))
  ;[0 0 0] Attach to gun
  (bind _asbp_gun (cast `/Game/VR_Weapons/Global/Blueprints/BP_Gun` OtherActor))
  (if (and (`|EnumEquality` (`/Game/VR_Weapons/Global/Blueprints/BP_Gun.Weapon` _asbp_gun) (`self.Weapon Type`)) (`ActorComponent.ComponentHasTag` OtherComp "Silencer") (`self.Silencer ready`) (== (`/Game/VR_Weapons/Global/Blueprints/BP_Gun.Silencer` _asbp_gun) false))
    (bind _automatic_shots_sound (`/Game/VR_Weapons/Global/Blueprints/BP_Gun.Automatic shots sound` _asbp_gun))
    (if (`KismetSystemLibrary.IsValid` _automatic_shots_sound)
      (if (not (`AudioComponent.IsPlaying` _automatic_shots_sound))
        (set `self.BP_gun` _asbp_gun :!label _label) ; create bp gun reference
        (`self.K2_DetachFromActor` "KeepWorld" "KeepWorld" "KeepWorld") ; detach from hand
        (bind _returnvalue (`SceneComponent.K2_AttachToComponent` (`self.Silencer`) (`/Game/VR_Weapons/Global/Blueprints/BP_Gun.Gun mesh` (`self.BP_gun`)) "Silencer" "SnapToTarget" "SnapToTarget" "SnapToTarget" true)) ; attach to gun
        (if _returnvalue
          (`/Game/VR_Weapons/Global/Blueprints/BP_Gun.Silencer attached` (`self.BP_gun`))
          (`GameplayStatics.PlaySoundAtLocation` "/Game/VR_Weapons/Global/Audio/Silencer_attach_Cue.Silencer_attach_Cue" (`SceneComponent.K2_GetComponentLocation` (`self.Collision`)) (struct) 1.0 1.0 0.0 "/Game/VR_Weapons/Global/Audio/Small_object_Attenuation.Small_object_Attenuation" null null)
          (`self.Change grip in anim BP when silencer is not in hand`)))
      (else
        (goto _label)))))

(event `/Game/VR_Weapons/Pawn/Blueprints/PickupActorInterface.Drop`
  ;[0 0 0] Drop
  (`PrimitiveComponent.SetSimulatePhysics` (`self.Silencer`) true)
  (`self.K2_DetachFromActor` "KeepWorld" "KeepWorld" "KeepWorld")
  (`self.Change grip in anim BP when silencer is not in hand`))

(event `Silencer ready event`
  (set `self.Silencer ready` false)
  (`KismetSystemLibrary.Delay` 0.5)
  (set `self.Silencer ready` true))

(fn `GripHandGuard`
  (params (Hand :type "/Game/VR_Weapons/Pawn/Blueprints/BP_MotionController Object Reference"))
  (returns (HandguardGrabbed :type Boolean))
  (return false))

(fn `InsertMagazine`
  (params (OverlappedComponent :type "PrimitiveComponent Object Reference") (WeaponType :type "/Game/VR_Weapons/Pawn/Blueprints/E_WeaponType Enum" :default "NewEnumerator0"))
  (returns (`Magazine Compatible` :type Boolean) (`Weapon Mesh` :type "StaticMeshComponent Object Reference") (`Weapon Actor` :type "/Game/VR_Weapons/Global/Blueprints/BP_Gun Object Reference"))
  (return false null null))

(fn `Pickup`
  (params (Hand :type "EControllerHand Enum" :default "Left") (`Grip or grab` :type "/Game/VR_Weapons/Pawn/Blueprints/E_GrabType Enum" :default "NewEnumerator1") (Actor :type "/Game/VR_Weapons/Pawn/Blueprints/BP_MotionController Object Reference") (AttachTo :type "SceneComponent Object Reference"))
  (returns (WeaponType :type "/Game/VR_Weapons/Pawn/Blueprints/E_WeaponType Enum") (GunGrabbed :type Boolean))
  (bind _bp_gun (`self.BP_gun`))
  (bind _weapon_type (`self.Weapon Type`))
  (switch `/Game/VR_Weapons/Pawn/Blueprints/E_GrabType` `Grip or grab`
    (:`NewEnumerator1`
      (`self.Silencer ready event`)
      ;[0 0 0] Switch to silencer grip in Anim BP
      (bind _asright_hand_anim_bp (cast `/Game/VR_Weapons/Pawn/Mannequin/Animations/RightHand_AnimBP` (`SkeletalMeshComponent.GetAnimInstance` (`/Game/VR_Weapons/Pawn/Blueprints/BP_MotionController.HandMesh` Actor))))
      (set `/Game/VR_Weapons/Pawn/Mannequin/Animations/RightHand_AnimBP.Silencer` true _asright_hand_anim_bp)
      (set `/Game/VR_Weapons/Pawn/Mannequin/Animations/RightHand_AnimBP.Grip` 1.0 _asright_hand_anim_bp)
      (set `/Game/VR_Weapons/Pawn/Mannequin/Animations/RightHand_AnimBP.Weapon` (`KismetMathLibrary.Conv_ByteToDouble` _weapon_type) _asright_hand_anim_bp)
      (set `self.BP_MotionController` Actor)
      (`PrimitiveComponent.SetSimulatePhysics` (`self.Silencer`) false)
      (bind _returnvalue (`SceneComponent.K2_AttachToComponent` (`self.K2_GetRootComponent`) AttachTo (select `bool` (`|EnumEquality` _weapon_type "NewEnumerator4") :`false` "SilencerGripSocket" :`true` "SilencerHandgunGripSocket" :!type "Name") "SnapToTarget" "SnapToTarget" "SnapToTarget" true))
      (`KismetSystemLibrary.PrintString` (`KismetStringLibrary.Conv_BoolToString` _returnvalue) true true (struct :`R` 1.0 :`G` 0.467875 :`A` 1.0))
      (`|ExecutionSequence`
        (:`then_0`
          (`/Engine/EditorBlueprintResources/StandardMacros.IsValid` _bp_gun
            (:`Is Valid`
              (set `/Game/VR_Weapons/Global/Blueprints/BP_Gun.Silencer` false _bp_gun) ; update BPgun that the silencer has been removed
            )))
        (:`then_1`
          (return "NewEnumerator0" false))))))

(fn `PullTrigger`
  (returns (Fired :type Boolean))
  (return false))

(fn `UserConstructionScript`)