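; VR weapon magazine actor that a motion-controller hand grabs, drops and inserts into compatible guns.
; Pickup attaches it to a type-specific hand socket and clears the gun's magazine reference.
; Insert overlap checks compatibility via interface message, then snaps it to the weapon with sound and haptics, using a ready flag against instant re-attachment.
; Cartridge meshes track rounds, optionally as instanced meshes, and empty magazines can spawn replacements when dropped.
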(event `self.ReceiveBeginPlay`
  (`PrimitiveComponent.SetSimulatePhysics` (`self.Magazine`) (`self.Start simulating physics`)))

(event `Pickup_Event`
  (params (`Grip or Grab` :type "/Game/VR_Weapons/Pawn/Blueprints/E_GrabType Enum" :default "NewEnumerator1") (MotionController :type "/Game/VR_Weapons/Pawn/Blueprints/BP_MotionController Object Reference") (HandMesh :type "SceneComponent Object Reference"))
  (bind _debug_mode (`self.Debug mode`))
  (bind _debug_mode_2 (`self.Debug mode`))
  (bind _weaponbp (`self.WeaponBP`))
  (bind _debug_mode_3 (`self.Debug mode`))
  (bind _debug_mode_4 (`self.Debug mode`))
  (`KismetSystemLibrary.PrintString` "Mag pick-up event" _debug_mode_4 _debug_mode_4)
  (if (`|EnumEquality` `Grip or Grab` "NewEnumerator1")
    (bind _output_get (set `self.MotionController` MotionController))
    (set `/Game/VR_Weapons/Pawn/Blueprints/BP_MotionController.Weapon` (`self.MagazineType`) _output_get) ; Set weapon to engage to update \nblendspace anim
    (set `/Game/VR_Weapons/Pawn/Blueprints/BP_MotionController.Engage` true _output_get) ; Set hand to engage to update \nblendspace anim
    (`KismetSystemLibrary.PrintString` "pick up mag" _debug_mode_2 _debug_mode_2 (struct :`R` 0.150572 :`G` 1.0 :`A` 1.0) 3.0)
    (`PrimitiveComponent.SetSimulatePhysics` (`self.Magazine`) false)
    (bind _returnvalue (`SceneComponent.K2_AttachToComponent` (`self.K2_GetRootComponent`) HandMesh (select `/Game/VR_Weapons/Pawn/Blueprints/E_WeaponType` (`self.MagazineType`) :`NewEnumerator4` "Handgun_MagazineGripSocket" :`NewEnumerator1` "Sub-machine_gun_MagazineGripSocket" :`NewEnumerator5` "Assault_rifle_MagazineGripSocket" :`NewEnumerator3` "Sniper_rifle_MagazineGripSocket" :!type "Name") "SnapToTarget" "SnapToTarget" "SnapToTarget" true))
    (set `self.Magazine ready to load` false) ; Stop it instantly re-attaching when removed from gun
    (`|ExecutionSequence`
      (:`then_1`
        (`KismetSystemLibrary.Delay` 0.25)
        (set `self.Magazine ready to load` true) ; allow the user to grab the mag \nwithout it instantly re-attaching
      )
      (:`then_2`
        (if _returnvalue
          (`KismetSystemLibrary.PrintString` "Mag picked up" _debug_mode_3 _debug_mode_3 (struct :`R` 0.032452 :`G` 1.0 :`A` 1.0))
          (`/Engine/EditorBlueprintResources/StandardMacros.IsValid` _weaponbp
            (:`Is Valid`
              (`GameplayStatics.PlaySoundAtLocation` (`self.Magazine out audio`) (`SceneComponent.K2_GetComponentLocation` (`self.Magazine`)) (struct) 1.0 1.0 0.0 "/Game/VR_Weapons/Global/Audio/Weapon_Attenuation.Weapon_Attenuation" null null) ; click sound effect
              (set `/Game/VR_Weapons/Global/Blueprints/BP_Gun.Magazine` null _weaponbp) ; when magazine is picked up it is no longer attached to the gun, \ntherefore destroy magazine reference in WeaponBP to disable firing
            ))
          (else
            (`KismetSystemLibrary.PrintString` "Mag not picked up" _debug_mode_3 _debug_mode_3 (struct :`R` 1.0 :`G` 0.046875 :`B` 0.046875 :`A` 1.0))))))
    (else
      (`KismetSystemLibrary.PrintString` "Hand is not grabbing" _debug_mode _debug_mode (struct :`R` 1.0 :`G` 0.078125 :`B` 0.097978 :`A` 1.0)))))

(event `/Game/VR_Weapons/Pawn/Blueprints/PickupActorInterface.Drop`
  (bind _motioncontroller (`self.MotionController`))
  (set `/Game/VR_Weapons/Pawn/Blueprints/BP_MotionController.Weapon` "NewEnumerator0" _motioncontroller)
  (set `/Game/VR_Weapons/Pawn/Blueprints/BP_MotionController.Engage` false _motioncontroller)
  (`PrimitiveComponent.SetSimulatePhysics` (`self.Magazine`) true)
  (`self.K2_DetachFromActor` "KeepWorld" "KeepWorld" "KeepWorld")
  (if (and (`self.Autospawn new magazine`) (== (`self.Rounds`) 0))
    (`KismetSystemLibrary.Delay` 0.1)
    (`|SpawnActorFromClass` (`GameplayStatics.GetObjectClass` self) (`KismetMathLibrary.MakeTransform` (`KismetMathLibrary.MakeVector` (.x (.location (`self.GetTransform`))) (.y (.location (`self.GetTransform`))) (+ (.z (.location (`self.GetTransform`))) 10.0)) (.rotation (`self.GetTransform`)) (.scale (`self.GetTransform`))) "Undefined" "OverrideRootScale" null 30 false (`self.Autospawn new magazine`) null) ; Spawn a new magazine of this type
  ))

(event `self.InsertCollision.OnComponentBeginOverlap`
  (params (OverlappedComponent :type "PrimitiveComponent Object Reference") (OtherActor :type "Actor Object Reference") (OtherComp :type "PrimitiveComponent Object Reference") (OtherBodyIndex :type Integer) (bFromSweep :type Boolean) (SweepResult :type "HitResult Structure (by ref)"))
  (bind _debug_mode (`self.Debug mode`))
  (bind _debug_mode_2 (`self.Debug mode`))
  (bind _magazine_ready_to_load (`self.Magazine ready to load`))
  (bind _debug_mode_3 (`self.Debug mode`))
  (bind _debug_mode_4 (`self.Debug mode`))
  (bind _motioncontroller (`self.MotionController`))
  (bind _magazine (`self.Magazine`))
  (`KismetSystemLibrary.Delay` 0.1)
  (bind (_magazine_compatible _weapon_mesh _weapon_actor) (message `/Game/VR_Weapons/Pawn/Blueprints/PickupActorInterface.InsertMagazine` OtherActor OtherComp (`self.MagazineType`) :!pinned true)) ; Try to send message to BP_gun to check magazine is compatible
  (if (and _magazine_compatible _magazine_ready_to_load)
    (if (not (`/Game/VR_Weapons/Global/Blueprints/BP_Gun.Weapon stored in utility belt` _weapon_actor))
      (bind _primary_motion_controller_bp (`/Game/VR_Weapons/Global/Blueprints/BP_Gun.Primary Motion Controller BP` _weapon_actor))
      (`/Engine/EditorBlueprintResources/StandardMacros.IsValid` _primary_motion_controller_bp
        (:`Is Valid`
          (`/Game/VR_Weapons/Pawn/Blueprints/BP_MotionController.RumbleController` _primary_motion_controller_bp "/Game/VR_Weapons/Pawn/Haptics/Haptics_single.Haptics_single" 0.4 false))
        (:`Is Not Valid`
          _))
      (bind _output_get (set `self.WeaponBP` _weapon_actor))
      (set `/Game/VR_Weapons/Global/Blueprints/BP_Gun.Magazine` self _output_get)
      (set `self.MagazineWell` OtherComp)
      (`KismetSystemLibrary.PrintString` "compatible" _debug_mode _debug_mode (struct :`R` 0.242672 :`G` 1.0 :`A` 1.0))
      (`self.K2_DetachFromActor` "KeepWorld" "KeepWorld" "KeepWorld") ; detach from hand
      (bind _returnvalue (`SceneComponent.K2_AttachToComponent` _magazine _weapon_mesh "Magazine" "SnapToTarget" "SnapToTarget" "SnapToTarget" true)) ; attach to gun
      (if _returnvalue
        (set `self.Magazine ready to load` false)
        (`GameplayStatics.PlaySoundAtLocation` (`self.Magazine in audio`) (`SceneComponent.K2_GetComponentLocation` _magazine) (struct) 1.0 1.0 0.0 "/Game/VR_Weapons/Global/Audio/Weapon_Attenuation.Weapon_Attenuation" null null)
        (`KismetSystemLibrary.PrintString` "Magazine attached" _debug_mode_3 _debug_mode_3 (struct :`R` 0.452687 :`G` 1.0 :`A` 1.0))
        (`/Engine/EditorBlueprintResources/StandardMacros.IsValid` _motioncontroller
          (:`Is Valid`
            (`/Game/VR_Weapons/Pawn/Blueprints/BP_MotionController.RumbleController` _motioncontroller "/Game/VR_Weapons/Pawn/Haptics/Haptics_single.Haptics_single" 0.5 false)))
        (else
          (`KismetSystemLibrary.PrintString` "Magazine not attached" _debug_mode_4 _debug_mode_4 (struct :`R` 1.0 :`G` 0.056247 :`B` 0.03125 :`A` 1.0)))))
    (elif (not _magazine_ready_to_load)
      (`KismetSystemLibrary.PrintString` "magazine not ready to load" _debug_mode_2 _debug_mode_2 (struct :`R` 1.0 :`G` 0.020833 :`B` 0.064436 :`A` 1.0)))))

(event `self.InsertCollision.OnComponentEndOverlap`
  (params (OverlappedComponent :type "PrimitiveComponent Object Reference") (OtherActor :type "Actor Object Reference") (OtherComp :type "PrimitiveComponent Object Reference") (OtherBodyIndex :type Integer))
  (if (== OtherComp (`self.MagazineWell`))
    (`KismetSystemLibrary.Delay` 0.25)
    (set `self.Magazine ready to load` true)))

(fn `GripHandGuard`
  (params (Hand :type "/Game/VR_Weapons/Pawn/Blueprints/BP_MotionController Object Reference"))
  (returns (HandguardGrabbed :type Boolean))
  (return false))

(fn `InsertMagazine`
  (params (OverlappedComponent :type "PrimitiveComponent Object Reference") (WeaponType :type "/Game/VR_Weapons/Pawn/Blueprints/E_WeaponType Enum" :default "NewEnumerator0"))
  (returns (`Magazine Compatible` :type Boolean) (`Weapon Mesh` :type "StaticMeshComponent Object Reference") (`Weapon Actor` :type "/Game/VR_Weapons/Global/Blueprints/BP_Gun Object Reference"))
  (return false null null))

(fn `Pickup`
  (params (Hand :type "EControllerHand Enum" :default "Left") (`Grip or grab` :type "/Game/VR_Weapons/Pawn/Blueprints/E_GrabType Enum" :default "NewEnumerator1") (Actor :type "/Game/VR_Weapons/Pawn/Blueprints/BP_MotionController Object Reference") (AttachTo :type "SceneComponent Object Reference"))
  (returns (WeaponType :type "/Game/VR_Weapons/Pawn/Blueprints/E_WeaponType Enum") (GunGrabbed :type Boolean))
  (`self.Pickup_Event` `Grip or grab` Actor AttachTo)
  (return (`self.MagazineType`) false))

(fn `PullTrigger`
  (returns (Fired :type Boolean))
  (return false))

(fn `Remove round`
  (bind _ism_cartridge (`self.ISM cartridge`))
  (bind _rounds (`self.Rounds`))
  (bind _output (`|GetArrayItem` (`self.Cartridge meshes`) (`self.Rounds`)))
  (set `self.Rounds` (- (`self.Rounds`) 1))
  (if (`self.Use ISM cartridges`)
    (if (<= _rounds (`InstancedStaticMeshComponent.GetInstanceCount` _ism_cartridge))
      (`InstancedStaticMeshComponent.RemoveInstance` _ism_cartridge _rounds))
    (else
      (`/Engine/EditorBlueprintResources/StandardMacros.IsValid` _output
        (:`Is Valid`
          (`ActorComponent.K2_DestroyComponent` _output))))))

(fn `UserConstructionScript`
  (`SceneComponent.SetHiddenInGame` (`self.PickupCollision`) (not (`self.Debug mode`)) false)
  (`SceneComponent.SetHiddenInGame` (`self.InsertCollision`) (not (`self.Debug mode`)) false)
  (if (`self.Use ISM cartridges`)
    ;[0 0 0] replace all bullet mesh components with instanced static meshes to reduce draw calls
    (for (_array_element _array_index) (`self.Cartridge meshes`)
      (if (not (>= _array_index (`self.Rounds`)))
        (`InstancedStaticMeshComponent.AddInstance` (`self.ISM cartridge`) (`KismetMathLibrary.MakeTransform` (`SceneComponent.RelativeLocation` _array_element) (`SceneComponent.RelativeRotation` _array_element))))
      (`ActorComponent.K2_DestroyComponent` _array_element))
    (else
      ;[0 0 0] Remove additional cartridge meshes if the number of rounds is lowered
      (for _index (range (`self.Rounds`) (+ (`KismetArrayLibrary.Array_Length` (`self.Cartridge meshes`)) 1))
        (`ActorComponent.K2_DestroyComponent` (`|GetArrayItem` (`self.Cartridge meshes`) _index))))))