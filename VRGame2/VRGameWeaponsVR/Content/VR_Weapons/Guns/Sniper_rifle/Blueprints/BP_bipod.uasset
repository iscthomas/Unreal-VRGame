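; VR bipod actor that a sniper rifle mounts on, tracking the gripping motion controller to aim and slide the gun.
; Each Tick while gripped, the pivot looks along the controller-to-pivot line and controller distance drives the slider rail.
; Leaving the rail range reattaches the gun to the hand and destroys the bipod.
; A timeline adds recoil, and a fake rifle-attached hand replaces the real hand mesh while mounted.
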(event `Recoil`
  (bind _debug (`self.Debug`))
  ;[0 0 0] Recoil
  (`KismetSystemLibrary.PrintString` "Hello" _debug _debug (struct :`R` 0.123603 :`G` 1.0 :`A` 1.0) 3.0)
  (bind (_direction _bipod _slider_rail) (`Timeline|Bipod recoil` :!via `PlayFromStart`)
    (:`Update`
      (`self.K2_SetActorLocation` (+ (* (`KismetMathLibrary.Conv_RotatorToVector` (`SceneComponent.K2_GetComponentRotation` (`self.Pivot`))) _bipod) (`self.K2_GetActorLocation`)))
      (set `self.Slider rail offset` _slider_rail))))

(event `self.ReceiveTick`
  (params (DeltaSeconds :type "Float (single-precision)"))
  (bind _debug (`self.Debug`))
  (bind _bp_gun (`self.BP gun`))
  (bind _relativelocation_x (`KismetMathLibrary.BreakVector` (`SceneComponent.RelativeLocation` (`self.Slider Rail dummy`))))
  (bind _returnvalue (- (`self.Starting distance`) (`KismetMathLibrary.Vector_Distance` (`SceneComponent.K2_GetComponentLocation` (`self.MotionController`)) (`SceneComponent.K2_GetComponentLocation` (`self.Pivot`)))))
  ;[0 0 0] Update gun position by rotating the pivot and moving the slider rail
  ; (calculated by measuring look at rotation and distance between motion controller and pivot)
  (`/Engine/EditorBlueprintResources/StandardMacros.IsValid` (`self.MotionController`)
    (:`Is Valid`
      (switch `/Game/VR_Weapons/Pawn/Blueprints/E_GripEnum` (`/Game/VR_Weapons/Pawn/Blueprints/BP_MotionController.GripState` (`self.MotionControllerBP`))
        (:`NewEnumerator0`
          (`/Engine/EditorBlueprintResources/StandardMacros.DoOnce` false :!label _label
            (:`Completed`
              (set `self.MotionController` null) ; clear reference when user releases grip
            )))
        (:`NewEnumerator1`
          (goto _label))
        (:`NewEnumerator2`
          (`|ExecutionSequence` :!label _label_2
            (:`then_0`
              (goto _label :!via `Reset`))
            (:`then_1`
              (`SceneComponent.K2_SetWorldRotation` (`self.Pivot`) (`KismetMathLibrary.FindLookAtRotation` (+ (`SceneComponent.K2_GetComponentLocation` (`self.MotionController`)) (0.0 0.0 2.0)) (`SceneComponent.K2_GetComponentLocation` (`self.Pivot`))) false false)
              (`SceneComponent.K2_SetRelativeLocation` (`self.Slider Rail dummy`) (`KismetMathLibrary.MakeVector` (- _returnvalue (`self.Slider rail offset`))) false false)
              (`KismetSystemLibrary.PrintString` (`KismetStringLibrary.Concat_StrStr` "---- Sliderbar location: " (`KismetStringLibrary.Conv_DoubleToString` _returnvalue) " \n----Mounted = " (`KismetStringLibrary.Conv_BoolToString` (`self.Mounted`))) _debug _debug (struct :`R` 1.0 :`G` 0.227956 :`B` 0.208059 :`A` 1.0) 0.0)
              (if (and (or (< _returnvalue 0.5) (> _returnvalue 24.0)) (`self.Mounted`))
                ;[0 0 0] remove gun from bipod
                (set `/Game/VR_Weapons/Global/Blueprints/BP_Gun.Bipod` null (`self.BP gun`)) ; clear reference
                (`SceneComponent.K2_AttachToComponent` (`self.K2_GetRootComponent` _bp_gun) (`/Game/VR_Weapons/Pawn/Blueprints/BP_MotionController.HandMesh` (`self.MotionControllerBP`)) (select `/Game/VR_Weapons/Pawn/Blueprints/E_WeaponType` (`/Game/VR_Weapons/Global/Blueprints/BP_Gun.Weapon` _bp_gun) :`NewEnumerator3` "Sniper_rifle_GripSocket" :!type "Name") "SnapToTarget" "SnapToTarget" "SnapToTarget" true)
                (`/Game/VR_Weapons/Pawn/Blueprints/BP_MotionController.RumbleController` (`self.MotionControllerBP`) "/Game/VR_Weapons/Pawn/Haptics/Haptics_single.Haptics_single" 0.5 false)
                (bind _asbp_sniper_rifle (cast `/Game/VR_Weapons/Guns/Sniper_rifle/Blueprints/BP_Sniper_rifle` (`self.BP gun`)))
                (`/Game/VR_Weapons/Guns/Sniper_rifle/Blueprints/BP_Sniper_rifle.Removed from bipod` _asbp_sniper_rifle)
                (`/Game/VR_Weapons/Guns/Sniper_rifle/Blueprints/BP_Sniper_rifle.Bipod destroyed` _asbp_sniper_rifle _relativelocation_x)
                (`self.Update hand mesh visibility` true) ; Show motion controller hand mesh and hide fake hand mesh
                (`self.K2_DestroyActor`)))))
        (:`NewEnumerator4`
          (goto _label_2))))))

(event `Bipod spawned`
  (params (`BP gun` :type "/Game/VR_Weapons/Global/Blueprints/BP_Gun Object Reference"))
  ;[0 0 0] Mount gun on bipod when gun overlaps with valid surface
  (`self.Mount gun` `BP gun`))

(event `Grab mounted gun`
  (params (BP_weapon :type "/Game/VR_Weapons/Global/Blueprints/BP_Gun Object Reference") (Hand :type "EControllerHand Enum" :default "Left"))
  ;[0 0 0] Grab gun while its mounted on bipod
  (`self.Grab gun while mounted` BP_weapon Hand))

(fn `Grab gun while mounted`
  (params (BP_gun_ref :type "/Game/VR_Weapons/Global/Blueprints/BP_Gun Object Reference") (Hand :type "EControllerHand Enum" :default "Left"))
  (bind _bp_gun_ref (`local.BP_gun_ref`))
  (bind _primary_motion_controller_bp (`/Game/VR_Weapons/Global/Blueprints/BP_Gun.Primary Motion Controller BP` _bp_gun_ref))
  (`KismetSystemLibrary.PrintString` "Grabbing gun while mounted" true true (struct :`G` 0.66 :`B` 1.0 :`A` 1.0) 5.0)
  (`self.SetActorScale3D` (`local.BP_gun_ref`) (select `bool` (`|EnumEquality` Hand "Left") :`false` (1.0 1.0 1.0) :`true` (1.0 -1.0 1.0) :!type "Vector Structure")) ; flip sniper if left hand is grabbing
  (bind _asbp_sniper_rifle (cast `/Game/VR_Weapons/Guns/Sniper_rifle/Blueprints/BP_Sniper_rifle` (`local.BP_gun_ref`))
    (:`then`
      (`/Game/VR_Weapons/Guns/Sniper_rifle/Blueprints/BP_Sniper_rifle.Mounted sniper grabbed` _asbp_sniper_rifle))
    (:`CastFailed`
      _))
  (bind _output_get (set `self.BP gun` _bp_gun_ref)) ; Set BP gun reference
  (set `/Game/VR_Weapons/Global/Blueprints/BP_Gun.Bipod` self _output_get) ; Set bipod reference in BP gun
  (set `self.MotionControllerBP` _primary_motion_controller_bp) ; Set motion controller actor reference
  (set `self.MotionController` (`/Game/VR_Weapons/Pawn/Blueprints/BP_MotionController.MotionController` _primary_motion_controller_bp)) ; Set motion controller component  reference
  (`self.Update hand mesh visibility` false) ; Hide motion controller hand mesh and show fake hand mesh
)

(fn `Mount gun`
  (params (`BP gun` :type "/Game/VR_Weapons/Global/Blueprints/BP_Gun Object Reference"))
  (bind _debug (`self.Debug`))
  (bind _primary_motion_controller_bp (`/Game/VR_Weapons/Global/Blueprints/BP_Gun.Primary Motion Controller BP` `BP gun`))
  (bind _motioncontrollerbp (`self.MotionControllerBP`))
  (bind _debug_2 (`self.Debug`))
  (if (not (`self.Mounted`))
    (set `self.Mounted` true)
    (`SceneComponent.K2_SetRelativeLocation` (`self.Slider Rail dummy`) (`KismetMathLibrary.MakeVector` (`KismetMathLibrary.Vector_Distance2D` (`SceneComponent.K2_GetComponentLocation` (`self.Slider Rail dummy`)) (`SceneComponent.GetSocketLocation` (`/Game/VR_Weapons/Global/Blueprints/BP_Gun.Gun mesh` `BP gun`) "Bipod"))) false false) ; set slider rail position so its underneath the gun's "bipod" socket
    (`self.K2_AttachToComponent` `BP gun` (`self.Attach dummy`) "None" "SnapToTarget" "SnapToTarget" "KeepRelative" true) ; Attach gun to the "Attach dummy". \n\nThis positions the gun correctly on the bipod. \n\nThe Attach dummy is attached to the Slider rail and Pivot \nso the gun can be moved forward/back and rotated up/down/left/right
    (`KismetSystemLibrary.PrintString` "attach" _debug _debug (struct :`R` 0.003254 :`G` 1.0 :`A` 1.0))
    (`self.SetActorScale3D` (select `bool` (`|EnumEquality` (`/Game/VR_Weapons/Global/Blueprints/BP_Gun.Primary Hand` (`local.BP gun`)) "Left") :`false` (1.0 1.0 1.0) :`true` (1.0 -1.0 1.0) :!type "Vector Structure")) ; flip sniper if left hand is grabbing
    (bind _output_get (set `self.BP gun` `BP gun`)) ; Set BP gun reference
    (set `/Game/VR_Weapons/Global/Blueprints/BP_Gun.Bipod` self _output_get) ; Set bipod reference in BP gun
    (set `self.MotionControllerBP` _primary_motion_controller_bp) ; Set motion controller actor reference
    (`self.Update hand mesh visibility` false) ; Hide motion controller hand mesh and show fake hand mesh
    (bind _output_get_2 (set `self.MotionController` (`/Game/VR_Weapons/Pawn/Blueprints/BP_MotionController.MotionController` _primary_motion_controller_bp))) ; Set motion controller component  reference
    (set `self.Starting distance` (`KismetMathLibrary.Vector_Distance` (`SceneComponent.K2_GetComponentLocation` _output_get_2) (`SceneComponent.K2_GetComponentLocation` (`self.Slider Rail dummy`)))) ; Use this as a starting point to measure the motion controller movement
    (bind _asbp_sniper_rifle (cast `/Game/VR_Weapons/Guns/Sniper_rifle/Blueprints/BP_Sniper_rifle` (`self.BP gun`)))
    (`/Game/VR_Weapons/Guns/Sniper_rifle/Blueprints/BP_Sniper_rifle.Bipod mounted` _asbp_sniper_rifle)
    (`/Engine/EditorBlueprintResources/StandardMacros.IsValid` _motioncontrollerbp
      (:`Is Valid`
        (`/Game/VR_Weapons/Pawn/Blueprints/BP_MotionController.RumbleController` _motioncontrollerbp "/Game/VR_Weapons/Pawn/Haptics/Haptics_single.Haptics_single" 0.35 false) ; Vibrate motion controller
        (`KismetSystemLibrary.PrintString` "Rumble motion controller!" _debug_2 _debug_2 (struct :`R` 0.040787 :`G` 1.0 :`A` 1.0)))
      (:`Is Not Valid`
        (`KismetSystemLibrary.PrintString` "motion controller not valid" _debug_2 _debug_2 (struct :`R` 1.0 :`G` 0.03409 :`A` 1.0))))))

(fn `Update hand mesh visibility`
  (params (`Hand visibility` :type Boolean))
  (bind _motioncontrollerbp (`self.MotionControllerBP`))
  ;[0 0 0] Hides BP motion controller hand mesh. Then shows fake hand attached to rifle. This prevents the real hand mesh from rotating the wrong way and shows the hand mesh as always being aligned to the gun's pistol grip
  (`/Engine/EditorBlueprintResources/StandardMacros.IsValid` _motioncontrollerbp
    (:`Is Valid`
      (`SceneComponent.SetVisibility` (`/Game/VR_Weapons/Pawn/Blueprints/BP_MotionController.HandMesh` _motioncontrollerbp) `Hand visibility` false) ; Hide/show real motion controller mesh
      (bind _asbp_sniper_rifle (cast `/Game/VR_Weapons/Guns/Sniper_rifle/Blueprints/BP_Sniper_rifle` (`self.BP gun`)))
      (`SceneComponent.SetVisibility` (`/Game/VR_Weapons/Guns/Sniper_rifle/Blueprints/BP_Sniper_rifle.Bipod fakehand` _asbp_sniper_rifle) (not `Hand visibility`) false) ; Hide/show fake motion controller mesh
    )))

(fn `UserConstructionScript`)