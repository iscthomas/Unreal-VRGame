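; VR bolt-action sniper rifle Blueprint extending the base gun with a hand-operated bolt, attached scope and deployable bipod.
; Each tick maps hand movement to bolt rotation, then pull; cocking ejects the spent casing and chambers the next magazine round.
; Leg overlaps with line traces for flat static surfaces spawn a separate bipod actor.
; Scope render target flips according to primary hand and bipod mounting.
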(event `self.ReceiveBeginPlay`
  (`parent.ReceiveBeginPlay`)
  (`|ExecutionSequence`
    (:`then_0`
      (if (`self.Start simulating physics`)
        (`SceneComponent.K2_AttachToComponent` (`self.Bipod_mesh`) (`self.Gun mesh`) "None" "KeepWorld" "KeepWorld" "KeepWorld" true)))
    (:`then_1`
      ;[0 0 0] Called in parent BP_Gun
      (add `self.Weapon fired` (delegate `Weapon fired event`))
      (add `self.Weapon dropped` (delegate `Weapon dropped_Event`))
      (add `self.Weapon picked up` (delegate `Weapon picked up_Event`))
      (add `self.Weapon trigger pulled` (delegate `Weapon trigger pulled_Event`))
      (add `self.Weapon trigger released` (delegate `Weapon trigger released_Event`))
      ;[0 0 0] update animation of fake pistol grip hand
      (bind _asright_hand_anim_bp (cast `/Game/VR_Weapons/Pawn/Mannequin/Animations/RightHand_AnimBP` (`SkeletalMeshComponent.GetAnimInstance` (`self.Bipod fakehand`)) :!label _label))
      (set `/Game/VR_Weapons/Pawn/Mannequin/Animations/RightHand_AnimBP.GripState` "NewEnumerator2" _asright_hand_anim_bp) ; resting position
      (set `/Game/VR_Weapons/Pawn/Mannequin/Animations/RightHand_AnimBP.WeaponState` "NewEnumerator3" _asright_hand_anim_bp)
      (set `/Game/VR_Weapons/Pawn/Mannequin/Animations/RightHand_AnimBP.PrimaryGrip` true _asright_hand_anim_bp))))

(event `Weapon dropped_Event`
  ;[0 0 0] Attach/detach bipod to gun mesh when dropped (for collision purposes)
  (`SceneComponent.K2_AttachToComponent` (`self.Bipod_mesh`) (`self.Gun mesh`) "None" "KeepWorld" "KeepWorld" "KeepWorld" true)
  (`SceneComponent.SetVisibility` (`self.Bipod fakehand`) false false))

(event `Weapon picked up_Event`
  (bind _childactor (`ChildActorComponent.ChildActor` (`self.Scope`)))
  ;[0 0 0] Attach/detach bipod to gun mesh when dropped (for collision purposes)
  (`SceneComponent.K2_AttachToComponent` (`self.Bipod_mesh`) (`self.BipodPivot`) "None" "KeepWorld" "KeepWorld" "KeepWorld" true)
  (if (`self.Bipod ready`)
    (if (`|EnumEquality` (`self.Primary Hand`) "Left")
      (bind _asbp_scope (cast `/Game/VR_Weapons/Guns/Sniper_rifle/Blueprints/BP_scope` _childactor :!label _label_2))
      (bind _oculus_quest (`/Game/VR_Weapons/Global/Blueprints/GlobalFunctions.CheckDevice`))
      (`/Game/VR_Weapons/Guns/Sniper_rifle/Blueprints/BP_scope.Flip render target V` _asbp_scope (`KismetMathLibrary.SelectFloat` 1.0 -1.0 _oculus_quest))
      (`/Game/VR_Weapons/Guns/Sniper_rifle/Blueprints/BP_scope.Flip render target U` _asbp_scope 1.0)
      (else
        (bind _asbp_scope_2 (cast `/Game/VR_Weapons/Guns/Sniper_rifle/Blueprints/BP_scope` _childactor :!label _label_3))
        (bind _oculus_quest_2 (`/Game/VR_Weapons/Global/Blueprints/GlobalFunctions.CheckDevice`))
        (`/Game/VR_Weapons/Guns/Sniper_rifle/Blueprints/BP_scope.Flip render target V` _asbp_scope_2 (`KismetMathLibrary.SelectFloat` -1.0 1.0 _oculus_quest_2))
        (`/Game/VR_Weapons/Guns/Sniper_rifle/Blueprints/BP_scope.Flip render target U` _asbp_scope_2 1.0)))))

(event `Bipod mounted`
  (if (`|EnumEquality` (`self.Primary Hand`) "Left")
    (`|ExecutionSequence`
      (:`then_0`
        (goto _label_3))
      (:`then_1`
        (bind _asbp_scope (cast `/Game/VR_Weapons/Guns/Sniper_rifle/Blueprints/BP_scope` (`ChildActorComponent.ChildActor` (`self.Scope`)) :!label _label_4))
        (`/Game/VR_Weapons/Guns/Sniper_rifle/Blueprints/BP_scope.Flip render target U` _asbp_scope -1.0)))))

(event `Removed from bipod`
  (if (`|EnumEquality` (`self.Primary Hand`) "Left")
    (goto _label_2)))

(event `Mounted sniper grabbed`
  (if (`|EnumEquality` (`self.Primary Hand`) "Right")
    (bind _asbp_scope (cast `/Game/VR_Weapons/Guns/Sniper_rifle/Blueprints/BP_scope` (`ChildActorComponent.ChildActor` (`self.Scope`))))
    (`/Game/VR_Weapons/Guns/Sniper_rifle/Blueprints/BP_scope.Flip render target U` _asbp_scope 1.0)
    (else
      (goto _label_4))))

(event `Weapon trigger released_Event`
  ;[0 0 0] update animation of fake pistol grip hand
  (goto _label))

(event `Weapon trigger pulled_Event`
  ;[0 0 0] update animation of fake pistol grip hand
  (bind _asright_hand_anim_bp (cast `/Game/VR_Weapons/Pawn/Mannequin/Animations/RightHand_AnimBP` (`SkeletalMeshComponent.GetAnimInstance` (`self.Bipod fakehand`))))
  (set `/Game/VR_Weapons/Pawn/Mannequin/Animations/RightHand_AnimBP.GripState` "NewEnumerator4" _asright_hand_anim_bp) ; trigger pull
  (set `/Game/VR_Weapons/Pawn/Mannequin/Animations/RightHand_AnimBP.WeaponState` "NewEnumerator3" _asright_hand_anim_bp)
  (set `/Game/VR_Weapons/Pawn/Mannequin/Animations/RightHand_AnimBP.PrimaryGrip` true _asright_hand_anim_bp))

(event `Weapon fired event`
  (bind _bipod (`self.Bipod`))
  ;[0 0 0] Because this is a bolt action rifle the user must engage the charging handle after each shot
  (set `self.Weapon Cocked` false)
  (set `self.Shot fired` true)
  (`SceneComponent.SetVisibility` (`self.Casing`) true false)
  (`SceneComponent.SetVisibility` (`self.Chamber round`) false false)
  (`KismetSystemLibrary.PrintString` "Weapon fired Sucess" true true (struct :`R` 0.060965 :`G` 1.0 :`A` 1.0) 4.0)
  ;[0 0 0] Recoil
  (`/Engine/EditorBlueprintResources/StandardMacros.IsValid` _bipod ; Does bipod exist?
    (:`Is Valid`
      (`/Game/VR_Weapons/Guns/Sniper_rifle/Blueprints/BP_bipod.Recoil` _bipod) ; Bipod recoil animation
    )))

(event `self.ReceiveTick`
  (params (DeltaSeconds :type "Float (single-precision)"))
  (bind _magazine (`self.Magazine`))
  (bind _charging_handle_controller_bp (`self.Charging handle controller BP`))
  (bind _debug_mode (`self.Debug mode`))
  (bind _debug_mode_2 (`self.Debug mode`))
  (bind _debug_mode_3 (`self.Debug mode`))
  (bind _charging_handle_controller_bp_2 (`self.Charging handle controller BP`))
  (bind _charging_handle_controller_bp_3 (`self.Charging handle controller BP`))
  (bind _debug_mode_4 (`self.Debug mode`))
  (bind (_returnvalue_location _returnvalue_rotation) (`KismetMathLibrary.BreakTransform` (`SceneComponent.GetSocketTransform` (`self.Charging handle mesh`) "Shell" "RTS_World")))
  (bind _returnvalue (- (`self.Charging Handle distance`) 9.0))
  (bind (_relativelocation_x _relativelocation_y _relativelocation_z) (`KismetMathLibrary.BreakVector` (`SceneComponent.RelativeLocation` (`self.Charging handle collision`))))
  (bind _relativelocation_x_2 (`KismetMathLibrary.BreakVector` (`SceneComponent.RelativeLocation` (`self.Charging handle mesh`))))
  (bind _relativerotation_roll (`KismetMathLibrary.BreakRotator` (`SceneComponent.RelativeRotation` (`self.Charging handle mesh`))))
  (bind _relativerotation_roll_2 (`KismetMathLibrary.BreakRotator` (`SceneComponent.RelativeRotation` (`self.Charging handle mesh`))))
  (bind _returnvalue_2 (`KismetMathLibrary.FInterpTo_Constant` _relativelocation_x_2 0.0 DeltaSeconds 85.0))
  (bind _returnvalue_3 (`KismetMathLibrary.FClamp` _returnvalue -11.3 0.0))
  (bind _returnvalue_4 (and (`KismetSystemLibrary.IsValid` (`self.Bipod`)) (`KismetMathLibrary.NotEqualExactly_VectorVector` (`self.GetActorScale3D`) (1.0 1.0 1.0))))
  (bind _returnvalue_5 (`KismetMathLibrary.FClamp` (+ (* (- (`self.Bolt relative location`) (.z (`KismetMathLibrary.InverseTransformLocation` (`SceneComponent.K2_GetComponentToWorld` (`self.Gun mesh`)) (`SceneComponent.K2_GetComponentLocation` (`/Game/VR_Weapons/Pawn/Blueprints/BP_MotionController.GrabSphere` (`self.Charging handle controller BP`)))))) 8.0) 40.0) -60.0 0.0))
  ;[0 0 0] Custom behavior for cocking the bolt
  (`|ExecutionSequence`
    (:`then_0`
      (`/Engine/EditorBlueprintResources/StandardMacros.IsValid` (`self.Charging handle controller BP`)
        (:`Is Valid`
          (`KismetSystemLibrary.PrintString` "----- bolt hand valid" _debug_mode_4 _debug_mode_4 (struct :`R` 0.361059 :`G` 0.251376 :`B` 1.0 :`A` 1.0) DeltaSeconds)
          (if (`self.is Charging Handle grabbed`)
            (`|ExecutionSequence`
              (:`then_0`
                (`|ExecutionSequence`
                  (:`then_0`
                    (`/Engine/EditorBlueprintResources/StandardMacros.DoOnce` false :!label _label_5
                      (:`Completed`
                        (`self.Toggle charging handle fake hand` true)
                        (`/Game/VR_Weapons/Pawn/Blueprints/BP_MotionController.RumbleController` _charging_handle_controller_bp_2 "/Game/VR_Weapons/Pawn/Haptics/Haptics_single.Haptics_single" 0.4 false) ; initial grip vibration
                        (`KismetSystemLibrary.Delay` 0.2)
                        (`/Engine/EditorBlueprintResources/StandardMacros.IsValid` _charging_handle_controller_bp_2
                          (:`Is Valid`
                            (`/Game/VR_Weapons/Pawn/Blueprints/BP_MotionController.RumbleController` _charging_handle_controller_bp_2 "/Game/VR_Weapons/Pawn/Haptics/Haptics_auto.Haptics_auto" 0.2 true) ; sliding handle vibration
                          )
                          (:`Is Not Valid`
                            _))
                        (set `self.Charging Handle reset` true)
                        (`BoxComponent.SetBoxExtent` (`self.Charging handle collision`) (7.0 3.0 2.0) true) ; make collision box larger when grabbed so hand doesn't accidentally release too early
                        (`KismetSystemLibrary.PrintString` "-------------- Bolt grabbed" _debug_mode_2 _debug_mode_2 (struct :`R` 0.054149 :`G` 1.0 :`A` 1.0) 3.0))))
                  (:`then_1`
                    (goto _label_10 :!via `Reset`))))
              (:`then_1`
                (if (`self.is Charging Handle reset`)
                  (`|ExecutionSequence`
                    (:`then_0`
                      (set `self.Bolt relative location` _relativelocation_z) ; set bolt starting point on Z axis
                    )
                    (:`then_1`
                      (`|ExecutionSequence`
                        (:`then_0`
                          (`SceneComponent.K2_SetRelativeRotation` (`self.Charging handle mesh`) (`KismetMathLibrary.MakeRotator` _returnvalue_5) false false)
                          (`KismetSystemLibrary.PrintString` (`KismetStringLibrary.Conv_DoubleToString` _returnvalue_5) false false (struct :`R` 0.1057 :`B` 1.0 :`A` 1.0) 0.0)
                          (if (> _returnvalue_5 -30.0)
                            (goto _label_6 :!via `Reset`)))
                        (:`then_1`
                          (if (< _returnvalue_5 -55.0)
                            (`/Engine/EditorBlueprintResources/StandardMacros.DoOnce` false :!label _label_6 ; reset when bolt has been rotated in opposite direction
                              (:`Completed`
                                (`GameplayStatics.PlaySoundAtLocation` "/Game/VR_Weapons/Guns/Sniper_rifle/Audio/Sniper_rifle_bolt_grabbed_Cue.Sniper_rifle_bolt_grabbed_Cue" (`SceneComponent.K2_GetComponentLocation` (`self.Charging handle collision`)) (struct) 1.0 1.0 0.0 "/Game/VR_Weapons/Global/Audio/Weapon_Attenuation.Weapon_Attenuation" null null) ; click
                                (`/Game/VR_Weapons/Pawn/Blueprints/BP_MotionController.RumbleController` (`self.Charging handle controller BP`) "/Game/VR_Weapons/Pawn/Haptics/Haptics_single.Haptics_single" 0.6 false) ; vibration
                              )))))))))
              (:`then_2`
                (if (`self.is Charging Handle Fully rotated`)
                  (`|ExecutionSequence`
                    (:`then_0`
                      (set `self.Charging handle pull distance` _returnvalue)
                      (if (> _returnvalue -11.3)
                        (`SceneComponent.K2_SetRelativeLocation` (`self.Charging handle mesh`) (`KismetMathLibrary.MakeVector` _returnvalue_3) false false)
                        (`SceneComponent.K2_SetRelativeLocation` (`self.Safety mesh`) (`KismetMathLibrary.MakeVector` _returnvalue_3) false false)
                        (if (< _returnvalue -10.5)
                          (`KismetSystemLibrary.PrintString` "----------------- bolt cocked event -----------------" _debug_mode _debug_mode (struct :`G` 1.0 :`B` 0.003758 :`A` 1.0))
                          (if (`self.Charging Handle reset`)
                            (set `self.Charging Handle reset` false)
                            (`GameplayStatics.PlaySoundAtLocation` "/Game/VR_Weapons/Guns/Sniper_rifle/Audio/Sniper_rifle_bolt_cocked_Cue.Sniper_rifle_bolt_cocked_Cue" (`SceneComponent.K2_GetComponentLocation` (`self.Charging handle collision`)) (struct) 1.0 1.0 0.0 "/Game/VR_Weapons/Global/Audio/Small_object_Attenuation.Small_object_Attenuation" null null) ; cocked sound effect
                            (`self.Reset collision box extent`)
                            (`|ExecutionSequence`
                              (:`then_0`
                                (if (`self.Shot fired`)
                                  (`SceneComponent.SetVisibility` (`self.Casing`) false false) ; Hide casing mesh so particle effect \ncan animate it being ejected
                                  (bind _returnvalue_6 (`GameplayStatics.SpawnEmitterAtLocation` "/Game/VR_Weapons/Guns/Sniper_rifle/Particles/P_Sniper_rifle_Shell_ejections.P_Sniper_rifle_Shell_ejections" _returnvalue_location (`KismetMathLibrary.MakeRotator` (- (.roll _returnvalue_rotation) (`KismetMathLibrary.SelectFloat` 45.0 0.0 _returnvalue_4)) (.pitch _returnvalue_rotation) (- (.yaw _returnvalue_rotation) (`KismetMathLibrary.SelectFloat` 180.0 0.0 _returnvalue_4))))) ; Casing ejection particle emitter
                                  (`FXSystemComponent.SetVectorParameter` _returnvalue_6 "Mesh Rot" (`KismetMathLibrary.MakeVector` 0.0 0.0 (`self.Align mesh particle rotation with weapon` _returnvalue_rotation))) ; Orient mesh particle rotation correctly
                                  (add `ParticleSystemComponent.OnParticleCollide` _returnvalue_6 (delegate `Collision event`)) ; play sound when casing particles collides with object
                                  (set `self.Shot fired` false)))
                              (:`then_1`
                                (`/Engine/EditorBlueprintResources/StandardMacros.IsValid` _charging_handle_controller_bp
                                  (:`Is Valid`
                                    (`/Game/VR_Weapons/Pawn/Blueprints/BP_MotionController.RumbleController` _charging_handle_controller_bp "/Game/VR_Weapons/Pawn/Haptics/Haptics_single.Haptics_single" 0.7 false))))
                              (:`then_2`
                                (if (`KismetSystemLibrary.IsValid` _magazine)
                                  (if (> (`/Game/VR_Weapons/Global/Blueprints/BP_Magazine.Rounds` _magazine) 0)
                                    (set `self.Weapon Cocked` true) ; weapon is now cocked and ready to be shot
                                    (`self.Allow next bullet into chamber`)))))))
                        (else
                          (if (`self.is Charging Handle reset`) :!label _label_7
                            (`|ExecutionSequence`
                              (:`then_0`
                                (`/Engine/EditorBlueprintResources/StandardMacros.DoOnce` true :!label _label_8
                                  (:`Completed`
                                    (set `self.One in the chamber` true) ; Allow next bullet to be fired even without magazine loaded
                                    (`SceneComponent.SetVisibility` (`self.Chamber round`) true false) ; Make chamber bullet visible
                                    (`/Game/VR_Weapons/Global/Blueprints/BP_Magazine.Remove round` (`self.Magazine`)) ; bullet is now in chamber so remove bullet from the magazine
                                  )))
                              (:`then_1`
                                (if (== _relativerotation_roll 0.0)
                                  (`BoxComponent.SetBoxExtent` (`self.Charging handle collision`) (1.5 1.5 1.5) true) ; Rest collision box to normal size
                                  (else
                                    (`SceneComponent.K2_SetRelativeRotation` (`self.Charging handle mesh`) (`KismetMathLibrary.MakeRotator` (`KismetMathLibrary.FInterpTo_Constant` _relativerotation_roll 0.0 DeltaSeconds 600.0)) false false)))))
                            (else
                              (`SceneComponent.K2_SetRelativeLocation` (`self.Charging handle mesh`) (`KismetMathLibrary.MakeVector` _returnvalue_2) false false) ; Slide back to start location
                              (`SceneComponent.K2_SetRelativeLocation` (`self.Safety mesh`) (`KismetMathLibrary.MakeVector` _returnvalue_2) false false) ; Slide back to start location
                            )))))
                    (:`then_1`
                      (if (and (`self.Shot fired`) (< _returnvalue -2.5))
                        (`/Engine/EditorBlueprintResources/StandardMacros.DoOnce` false :!label _label_9
                          (:`Completed`
                            (`GameplayStatics.SpawnEmitterAttached` "/Game/VR_Weapons/Guns/Sniper_rifle/Particles/P_Sniper_rifle_ejector_smoke.P_Sniper_rifle_ejector_smoke" (`self.Charging handle mesh`) "Shell" (0.0 0.0 0.0) (struct) (1.0 1.0 1.0) "SnapToTarget") ; Spawn ejector smoke effect and attach it the bolt
                          ))))))))
            (else
              (`|ExecutionSequence`
                (:`then_0`
                  (`|ExecutionSequence`
                    (:`then_0`
                      (goto _label_5 :!via `Reset`))
                    (:`then_1`
                      (`/Engine/EditorBlueprintResources/StandardMacros.DoOnce` true :!label _label_10
                        (:`Completed`
                          (`self.Toggle charging handle fake hand` false)
                          (`KismetSystemLibrary.Delay` 0.2)
                          (`/Engine/EditorBlueprintResources/StandardMacros.IsValid` _charging_handle_controller_bp_3
                            (:`Is Valid`
                              (`PlayerController.StopHapticEffect` (`GameplayStatics.GetPlayerController` 0) (`/Game/VR_Weapons/Pawn/Blueprints/BP_MotionController.Hand` _charging_handle_controller_bp_3)) ; Stop sliding handle vibration
                              (`KismetSystemLibrary.PrintString` "-------------- Bolt released" _debug_mode_3 _debug_mode_3 (struct :`G` 1.0 :`B` 0.218392 :`A` 1.0) 3.0))))))))
                (:`then_1`
                  (goto _label_7))
                (:`then_2`
                  (`self.Reset collision box extent` :!label _label_11)
                  (goto _label_9 :!via `Reset`))))))
        (:`Is Not Valid`
          (if (and (`self.is Charging Handle reset`) (== _relativerotation_roll_2 0.0))
            (`KismetSystemLibrary.Delay` 0.1)
            (goto _label_11)
            (else
              (goto _label_7))))))
    (:`then_1`
      (`self.tick` DeltaSeconds)
      (`self.Gun aiming`))))

(event `Collision event`
  (params (EventName :type Name) (EmitterTime :type "Float (double-precision)") (ParticleTime :type Integer) (Location :type "Vector Structure") (Velocity :type "Vector Structure") (Direction :type "Vector Structure") (Normal :type "Vector Structure") (BoneName :type Name) (PhysMat :type "PhysicalMaterial Object Reference"))
  ;[0 0 0] Custom behavior for cocking the bolt
  (`/Engine/EditorBlueprintResources/StandardMacros.DoOnce` false :!label _label_12
    (:`Completed`
      (`GameplayStatics.PlaySoundAtLocation` (select `EPhysicalSurface` (`PhysicalMaterial.SurfaceType` PhysMat) :`SurfaceType_Default` "/Game/VR_Weapons/Guns/Sniper_rifle/Audio/Sniper_rifle_casing_default_hard_surface_Cue.Sniper_rifle_casing_default_hard_surface_Cue" :`SurfaceType1` "/Game/VR_Weapons/Guns/Sniper_rifle/Audio/Sniper_rifle_casing_default_hard_surface_Cue.Sniper_rifle_casing_default_hard_surface_Cue" :`SurfaceType2` "/Game/VR_Weapons/Guns/Sniper_rifle/Audio/Sniper_rifle_casing_wood_Cue.Sniper_rifle_casing_wood_Cue" :`SurfaceType3` "/Game/VR_Weapons/Guns/Sniper_rifle/Audio/Sniper_rifle_casing_default_hard_surface_Cue.Sniper_rifle_casing_default_hard_surface_Cue" :!type "SoundBase Object Reference") Location (struct) 1.0 1.0 0.0 "/Game/VR_Weapons/Global/Audio/Small_object_Attenuation.Small_object_Attenuation" null null) ; casing drop sound effect
      (`KismetSystemLibrary.Delay` 2.0)
      (goto _label_12 :!via `Reset`))))

(event `Allow next bullet into chamber`
  ;[0 0 0] Custom behavior for cocking the bolt
  (goto _label_8 :!via `Reset`))

(event `self.Right leg collision.OnComponentBeginOverlap`
  (params (OverlappedComponent :type "PrimitiveComponent Object Reference") (OtherActor :type "Actor Object Reference") (OtherComp :type "PrimitiveComponent Object Reference") (OtherBodyIndex :type Integer) (bFromSweep :type Boolean) (SweepResult :type "HitResult Structure (by ref)"))
  (bind (_returnvalue_roll _returnvalue_pitch _returnvalue_yaw) (`KismetMathLibrary.BreakRotator` (`SceneComponent.K2_GetComponentRotation` (`self.BipodPivot`))))
  ;[0 0 0] Mount on bipod
  (if (and (`self.Bipod ready`) (`KismetSystemLibrary.IsValid` (`self.Primary Motion Controller BP`)))
    (bind _returnvalue (`self.Check Surface Is Flat`))
    (if _returnvalue
      (`SceneComponent.SetVisibility` (`self.BipodPivot`) false true) ; hide bipod mesh
      (`PrimitiveComponent.SetCollisionEnabled` (`self.Charging handle collision`) "NoCollision") ; stop bolt being grabbed accidently while sniper is being mounted
      (bind _returnvalue_2 (`|SpawnActorFromClass` "/Game/VR_Weapons/Guns/Sniper_rifle/Blueprints/BP_bipod.BP_bipod_C" (`KismetMathLibrary.MakeTransform` (`self.Hit location`) (`KismetMathLibrary.MakeRotator` 0.0 0.0 _returnvalue_yaw)) "Undefined" "OverrideRootScale" null (`self.Debug mode`) null)) ; spawn bipod
      (`/Game/VR_Weapons/Guns/Sniper_rifle/Blueprints/BP_bipod.Bipod spawned` _returnvalue_2 self)
      (set `self.Bipod ready` false) ; Stop Bipod spawning unitl this one has been destroyed
      (`KismetSystemLibrary.Delay` 0.1)
      (`PrimitiveComponent.SetCollisionEnabled` (`self.Charging handle collision`) "QueryAndPhysics") ; Allow bolt to be grabbed after sniper is mounted
    )))

(event `tick`
  (params (DeltaTime :type "Float (double-precision)"))
  (bind _bipodpivot (`self.BipodPivot`))
  (bind _relativelocation_x (`KismetMathLibrary.BreakVector` (`SceneComponent.RelativeLocation` _bipodpivot)))
  ;[0 0 0] Move bipod back to start position when gun is lifted
  (if (!= (`SceneComponent.RelativeLocation` _bipodpivot) (0.0 0.0 0.0) :`ErrorTolerance` 0.001)
    (`SceneComponent.K2_SetRelativeLocation` (`self.BipodPivot`) (`KismetMathLibrary.MakeVector` (`KismetMathLibrary.FInterpTo` _relativelocation_x -10.0 DeltaTime 12.0)) false false)))

(event `Bipod destroyed`
  (params (`Slider rail position` :type "Float (double-precision)"))
  (`SceneComponent.K2_SetRelativeLocation` (`self.BipodPivot`) (`KismetMathLibrary.MakeVector` (* `Slider rail position` -1.0)) false false)
  (`SceneComponent.SetVisibility` (`self.BipodPivot`) true true)
  (`KismetSystemLibrary.Delay` 0.75)
  (set `self.Bipod ready` true))

(fn `Align mesh particle rotation with weapon`
  (params (InRot :type "Rotator Structure"))
  (returns (Rotation :type "Float (double-precision)"))
  (bind _yaw (.yaw InRot))
  (return (/ (+ (select `bool` (< _yaw 0.0) :`true` 360.0 :!type "Float (single-precision)") _yaw) 360.0)))

(fn `Check leg`
  (params (`trace start` :type "SceneComponent Object Reference"))
  (returns (ReturnValue :type Boolean))
  (locals (`surface flat` :type Boolean :default false))
  (bind _returnvalue (`SceneComponent.K2_GetComponentLocation` `trace start`))
  (bind (_outhit _returnvalue_2) (`KismetSystemLibrary.LineTraceSingle` :`Start` _returnvalue :`End` (- _returnvalue (0.0 0.0 8.0)) :`TraceChannel` "TraceTypeQuery1" :`DrawDebugType` (select `bool` (`self.Debug mode`) :`true` "ForDuration" :!type "EDrawDebugTrace Enum") :`DrawTime` 2.0))
  (bind _output_get (set `local.surface flat` _returnvalue_2))
  (if _output_get
    (bind (_bblockinghit _binitialoverlap _time _distance _location _impactpoint _normal _impactnormal _physmat _hitactor _hitcomponent) (`GameplayStatics.BreakHitResult` _outhit))
    (set `local.surface flat` (and (> (.z _normal) 0.95) _bblockinghit (`|EnumEquality` (`PrimitiveComponent.GetCollisionObjectType` _hitcomponent) "ECC_WorldStatic"))))
  (return (`local.surface flat`)))

(fn `Check Surface Is Flat`
  (returns (ReturnValue :type Boolean))
  (locals (flat :type Boolean))
  (bind _returnvalue (`SceneComponent.K2_GetComponentLocation` (`self.Bipod_mesh`)))
  (set `local.flat` false)
  (bind _returnvalue_2 (`self.Check leg` (`self.Left leg collision`)))
  (if _returnvalue_2
    (bind _returnvalue_3 (`self.Check leg` (`self.Right leg collision`)))
    (if _returnvalue_3
      (set `local.flat` true)
      (bind _outhit (`KismetSystemLibrary.LineTraceSingle` :`Start` _returnvalue :`End` (- _returnvalue (0.0 0.0 5.0)) :`TraceChannel` "TraceTypeQuery1" :`DrawDebugType` (select `bool` (`self.Debug mode`) :`true` "ForDuration" :!type "EDrawDebugTrace Enum") :`TraceColor` (struct :`G` 0.521003 :`B` 1.0 :`A` 1.0) :`TraceHitColor` (struct :`R` 0.021752 :`B` 1.0 :`A` 1.0) :`DrawTime` 2.0))
      (set `self.Hit location` (`.Location` (`GameplayStatics.BreakHitResult` _outhit)))
      (return (`local.flat`)))))

(fn `GripHandGuard`
  (params (Hand :type "/Game/VR_Weapons/Pawn/Blueprints/BP_MotionController Object Reference"))
  (returns (HandguardGrabbed :type Boolean))
  (`/Engine/EditorBlueprintResources/StandardMacros.IsValid` (`self.Bipod`) ; only grab handguard if not mounted on bipod
    (:`Is Valid`
      _)
    (:`Is Not Valid`
      (bind _handguardgrabbed (`parent.GripHandGuard` Hand))))
  (return _handguardgrabbed))

(fn `is Charging Handle Fully rotated`
  (returns (ReturnValue :type Boolean))
  (bind _relativerotation_roll (`KismetMathLibrary.BreakRotator` (`SceneComponent.RelativeRotation` (`self.Charging handle mesh`))))
  (return (< _relativerotation_roll -55.0)))

(fn `Is correct hand`
  (returns (ReturnValue :type Boolean))
  (return (not (`parent.Is correct hand`))))

(fn `Reset collision box extent`
  (`BoxComponent.SetBoxExtent` (`self.Charging handle collision`) (1.5 1.5 1.5) true) ; reset collision box
)

(fn `UserConstructionScript`
  (bind _gun_mesh (`self.Gun mesh`))
  (`parent.UserConstructionScript`)
  (set `self.Shell ejection emitter` null) ; keep this cleared as shell will be ejected manually\nwhen the bolt is cocked
  (`SceneComponent.K2_AttachToComponent` (`self.Charging handle mesh`) (`self.Bolt Dummy`) "None" "SnapToTarget" "KeepRelative" "KeepRelative" true)
  ;[0 0 0] Spawn and attach scope
  (bind _returnvalue (`AddComponent|NODE_AddChildActorComponent-0` :`RelativeTransform` (`SceneComponent.K2_GetComponentToWorld` _gun_mesh)))
  (bind _output_get (set `self.Scope` _returnvalue))
  (`SceneComponent.K2_AttachToComponent` _output_get _gun_mesh "Scope" "SnapToTarget" "SnapToTarget" "SnapToTarget" true)
  (`ActorComponent.K2_DestroyComponent` (`self.Ejector mesh`)))