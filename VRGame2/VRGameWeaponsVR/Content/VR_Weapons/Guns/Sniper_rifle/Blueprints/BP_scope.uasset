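; BP_scope is a VR sniper rifle scope that uses a SceneCaptureComponent2D for its lens view.
; BeginPlay caches the player's MotionControllerPawn camera and loops on a short delay, enabling every-frame capture only while the camera is near the recently rendered lens, saving render cost.
; The construction script creates a dynamic M_scope material instance, and two flip events set its U and V tiling parameters.
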(event `self.ReceiveBeginPlay`
  (bind _asmotion_controller_pawn (cast `/Game/VR_Weapons/Pawn/Blueprints/MotionControllerPawn` (`GameplayStatics.GetPlayerPawn` 0)))
  (set `self.Player camera` (`/Game/VR_Weapons/Pawn/Blueprints/MotionControllerPawn.Camera` _asmotion_controller_pawn))
  (`SceneCaptureComponent2D.CaptureScene` (`self.SceneCaptureComponent2D`))
  (`KismetSystemLibrary.Delay` 0.25 :!label _label)
  (set `SceneCaptureComponent.bCaptureEveryFrame` (and (< (`KismetMathLibrary.Vector_Distance` (`SceneComponent.K2_GetComponentLocation` (`self.Player camera`)) (`SceneComponent.K2_GetComponentLocation` (`self.Lens`))) 100.0) (`PrimitiveComponent.WasRecentlyRendered` (`self.Lens`) 0.1)) (`self.SceneCaptureComponent2D`))
  (goto _label))

(event `Flip render target V`
  (params (Value :type "Float (double-precision)"))
  (`MaterialInstanceDynamic.SetScalarParameterValue` (`self.Scope Material`) "Vtiling" Value))

(event `Flip render target U`
  (params (Value :type "Float (double-precision)"))
  (`MaterialInstanceDynamic.SetScalarParameterValue` (`self.Scope Material`) "Utiling" Value))

(fn `UserConstructionScript`
  (bind _returnvalue (`PrimitiveComponent.CreateDynamicMaterialInstance` (`self.SM_scope`) 1 "/Game/VR_Weapons/Guns/Sniper_rifle/Materials/M_scope.M_scope" "None"))
  (set `self.Scope Material` _returnvalue))