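; Magazine Blueprint for the VR sniper rifle, configuring an inherited magazine base for this weapon.
; The construction script sets the magazine type, insert and removal sound cues, and the cartridge mesh array before calling the parent construction script.
; A collapsed Make array graph references the .300 Winchester Magnum cartridge meshes for that array.
; The event graph holds only disabled or empty events, so no runtime logic is added here.
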(fn `UserConstructionScript`
  (set `self.MagazineType` "NewEnumerator3")
  (set `self.Magazine in audio` "/Game/VR_Weapons/Guns/Sniper_rifle/Audio/Sniper_rifle_magazine_in_Cue.Sniper_rifle_magazine_in_Cue")
  (set `self.Magazine out audio` "/Game/VR_Weapons/Guns/Sniper_rifle/Audio/Sniper_rifle_magazine_out_Cue.Sniper_rifle_magazine_out_Cue")
  (set `self.Cartridge meshes` (`|MakeArray` (`self.SM_300_Winchester_Magnum1`) (`self.SM_300_Winchester_Magnum2`) (`self.SM_300_Winchester_Magnum3`) (`self.SM_300_Winchester_Magnum4`) (`self.SM_300_Winchester_Magnum5`) (`self.SM_300_Winchester_Magnum6`) (`self.SM_300_Winchester_Magnum7`) (`self.SM_300_Winchester_Magnum8`) (`self.SM_300_Winchester_Magnum9`) (`self.SM_300_Winchester_Magnum10`)))
  (`parent.UserConstructionScript`))