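; VR assault rifle Blueprint that adds bolt lock-back, a bolt release paddle and swappable sights to its parent weapon.
; Firing the last round retracts the bolt; overlapping the paddle with a motion controller, while no secondary hand grips, releases it with haptics and sound, chambering a magazine round.
; Pickup mirrors the sight's Y scale by primary hand, and construction attaches the ejector to the charging handle and applies the sight mesh.
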(event `self.ReceiveBeginPlay`
  (`parent.ReceiveBeginPlay`)
  (add `self.Weapon fired` (delegate `Weapon fired_Event`))
  (add `self.Weapon picked up` (delegate `Weapon picked up_Event`)))

(event `Weapon fired_Event`
  (if (== (`/Game/VR_Weapons/Global/Blueprints/BP_Magazine.Rounds` (`self.Magazine`)) 0)
    (set `self.Bolt retracted` true)))

(event `Weapon picked up_Event`
  (bind _sm_sights (`self.SM_sights`))
  (switch `EControllerHand` (`self.Primary Hand`)
    (:`Left`
      (`SceneComponent.SetRelativeScale3D` _sm_sights (1.0 -1.0 1.0)) ; Un-flip the red dot sight when gun is grabbed with left hand
    )
    (:`Right`
      (`SceneComponent.SetRelativeScale3D` _sm_sights (1.0 1.0 1.0)))))

(event `self.Bolt catch/release paddle collision.OnComponentBeginOverlap`
  (params (OverlappedComponent :type "PrimitiveComponent Object Reference") (OtherActor :type "Actor Object Reference") (OtherComp :type "PrimitiveComponent Object Reference") (OtherBodyIndex :type Integer) (bFromSweep :type Boolean) (SweepResult :type "HitResult Structure (by ref)"))
  ;[0 0 0] Bolt catch/release paddle (an alternative to the charging handle when loading a new mag)
  (`/Engine/EditorBlueprintResources/StandardMacros.IsValid` (`self.Secondary Motion Controller BP`)
    (:`Is Not Valid`
      (bind _asbp_motion_controller (cast `/Game/VR_Weapons/Pawn/Blueprints/BP_MotionController` OtherActor))
      (if (and (`self.Bolt retracted`) (== (`self.Weapon Cocked`) false))
        (`/Engine/EditorBlueprintResources/StandardMacros.IsValid` (`self.Primary Motion Controller BP`)
          (:`Is Valid`
            (`/Game/VR_Weapons/Pawn/Blueprints/BP_MotionController.RumbleController` _asbp_motion_controller "/Game/VR_Weapons/Pawn/Haptics/Haptics_single.Haptics_single" 0.9 false)
            (`/Game/VR_Weapons/Pawn/Blueprints/BP_MotionController.RumbleController` (`self.Primary Motion Controller BP`) "/Game/VR_Weapons/Pawn/Haptics/Haptics_single.Haptics_single" 0.9 false))
          (:`Is Not Valid`
            _))
        (set `self.Bolt retracted` false)
        (`GameplayStatics.PlaySoundAtLocation` "/Game/VR_Weapons/Guns/Assault_rifle/Audio/Assault_rifle_charging_handle_release_Cue.Assault_rifle_charging_handle_release_Cue" (`SceneComponent.K2_GetComponentLocation` (`self.Charging handle collision`)) (struct) 1.0 1.0 0.0 "/Game/VR_Weapons/Global/Audio/Weapon_Attenuation.Weapon_Attenuation" "/Game/VR_Weapons/Global/Audio/WeaponConcurrency.WeaponConcurrency" null) ; Bolt click
        (`self.Load next round into chamber`) ; Load round from magazine into the chamber
        (if (`self.One in the chamber`)
          (`/Game/VR_Weapons/Global/Blueprints/BP_Magazine.Remove round` (`self.Magazine`)))))))

(event `Set sights`
  (params (NewMesh :type "StaticMesh Object Reference"))
  (`StaticMeshComponent.SetStaticMesh` (`self.SM_sights`) NewMesh))

(fn `UserConstructionScript`
  (`parent.UserConstructionScript`)
  (`SceneComponent.K2_AttachToComponent` (`self.Ejector mesh`) (`self.Charging handle mesh`) "None" "KeepWorld" "KeepWorld" "KeepWorld" true)
  (`StaticMeshComponent.SetStaticMesh` (`self.SM_sights`) (`self.Sights mesh`)))