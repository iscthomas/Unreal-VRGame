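; VR handgun weapon Blueprint that adds slide and barrel-tilt animation on top of its parent gun class.
; On the WeaponFired event, a timeline drives the slide and barrel, with a separate last-shot timeline plus ejector smoke when the chamber is empty.
; Tick interpolates the barrel toward its default transform while the gun is held and the charging handle is grabbed.
; The construction script removes the inherited ejector mesh.
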(event `self.ReceiveTick`
  (params (DeltaSeconds :type "Float (single-precision)"))
  (`parent.ReceiveTick` DeltaSeconds)
  (if (and (!= (`self.Primary Hand mesh`) null) (`self.Charging Handle Grabbed`))
    (`SceneComponent.K2_SetRelativeTransform` (`self.SM_handgun_barrel`) (`KismetMathLibrary.TInterpTo` (`SceneComponent.GetRelativeTransform` (`self.SM_handgun_barrel`)) (`self.Barrel default`) DeltaSeconds 75.0) false false)))

(event `self.ReceiveBeginPlay`
  (`parent.ReceiveBeginPlay`)
  (add `self.Weapon fired` (delegate `Weapon fired_Event`)))

(event `Weapon fired_Event`
  (bind _charging_handle_mesh (`self.Charging handle mesh`))
  (bind _charging_handle_mesh_2 (`self.Charging handle mesh`))
  (bind (_returnvalue_location _returnvalue_rotation) (`KismetMathLibrary.BreakTransform` (`SceneComponent.GetSocketTransform` _charging_handle_mesh "Ejector" "RTS_World")))
  (if (not (`self.One in the chamber`))
    (`GameplayStatics.SpawnEmitterAttached` "/Game/VR_Weapons/Guns/Handgun/Particles/P_Handgun_ejector_smoke_slide_retracted.P_Handgun_ejector_smoke_slide_retracted" _charging_handle_mesh "Ejector" _returnvalue_location _returnvalue_rotation (1.0 1.0 1.0) "KeepWorldPosition") ; spawn smoke particle
    ;[0 0 0] If last shot is being fired - keep slide fully retracted
    (bind (_direction _slide_position _barrel_tilt) (`Timeline|Last shot` :!via `PlayFromStart`)
      (:`Update`
        (`SceneComponent.K2_SetRelativeLocation` _charging_handle_mesh_2 (`KismetMathLibrary.MakeVector` _slide_position) false false) ; move slide back
        (`SceneComponent.K2_SetRelativeTransform` (`self.SM_handgun_barrel`) (`KismetMathLibrary.TLerp` (`self.Barrel default`) (`self.Barrel tilt`) _barrel_tilt) false false) ; tilt barrel upwards
      ))
    (else
      (bind (_direction_2 _slide_position_2 _barrel_slide) (`Timeline|Slide` :!via `PlayFromStart`)
        (:`Update`
          (`SceneComponent.K2_SetRelativeLocation` _charging_handle_mesh_2 (`KismetMathLibrary.MakeVector` _slide_position_2) false false) ; move slide back
          (`SceneComponent.K2_SetRelativeTransform` (`self.SM_handgun_barrel`) (`KismetMathLibrary.TLerp` (`self.Barrel default`) (`self.Barrel tilt`) _barrel_slide) false false) ; tilt barrel
        )))))

(fn `UserConstructionScript`
  (`parent.UserConstructionScript`)
  (`ActorComponent.K2_DestroyComponent` (`self.Ejector mesh`)))