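; BP_Magazine_shotgun is the magazine actor for the VR shotgun, tracking loaded rounds and showing them as cartridge meshes.
; On BeginPlay it registers itself with the shotgun and snaps its magazine component to the gun mesh's Magazine socket.
; Its construction script gathers seven cartridge meshes into an array.
; AddRound increments the count and places a cartridge offset by cartridge length, as either an instanced or regular static mesh.
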(event `self.ReceiveBeginPlay`
  (bind _bp_shotgun (`self.BP_Shotgun`))
  (`parent.ReceiveBeginPlay`)
  (set `/Game/VR_Weapons/Global/Blueprints/BP_Gun.Magazine` self _bp_shotgun)
  (`SceneComponent.K2_AttachToComponent` (`self.Magazine`) (`/Game/VR_Weapons/Global/Blueprints/BP_Gun.Gun mesh` _bp_shotgun) "Magazine" "SnapToTarget" "SnapToTarget" "SnapToTarget" true))

(fn `Add round`
  (locals (`Cartridge length` :type "Float (double-precision)" :default 6.9))
  (bind _output_get (set `self.Rounds` (+ (`self.Rounds`) 1)))
  (if (`self.Use ISM cartridges`)
    (bind _returnvalue (* (- _output_get 1) (`local.Cartridge length`)))
    (`InstancedStaticMeshComponent.AddInstance` (`self.ISM cartridge`) (`KismetMathLibrary.MakeTransform` (`KismetMathLibrary.MakeVector` _returnvalue)))
    (else
      (`AddComponent|NODE_AddStaticMeshComponent-0` :`RelativeTransform` (`KismetMathLibrary.MakeTransform` (`KismetMathLibrary.MakeVector` _returnvalue)))))
  (`KismetSystemLibrary.PrintString` "add round"))

(fn `UserConstructionScript`
  (set `self.Cartridge meshes` (`|MakeArray` (`self.SM_shotgun_cartridge1`) (`self.SM_shotgun_cartridge2`) (`self.SM_shotgun_cartridge3`) (`self.SM_shotgun_cartridge4`) (`self.SM_shotgun_cartridge5`) (`self.SM_shotgun_cartridge6`) (`self.SM_shotgun_cartridge7`)))
  (`parent.UserConstructionScript`))