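; VR pump-action shotgun, a child weapon Blueprint that spawns its own magazine and fires randomly spread pellet line traces.
; Tick drives the hand-pulled fore-end, which moves the bolt, ejects casings, chambers magazine rounds and must reset before firing.
; Fore-end velocity scales click sounds, haptics and casing ejection speed, while a post-shot timer keeps cartridges smoking.
; Also handles two-handed fore-end gripping and a construction-script pellet spread debug test.
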(event `self.ReceiveBeginPlay`
  ;[0 0 0] Spawn and attach magazine
  (`parent.ReceiveBeginPlay`)
  (`|SpawnActorFromClass` "/Game/VR_Weapons/Guns/Shotgun/Blueprints/BP_Magazine_shotgun.BP_Magazine_shotgun_C" (`SceneComponent.GetSocketTransform` (`self.Gun mesh`) "Magazine" "RTS_World") "Undefined" "OverrideRootScale" null self (`self.Magazine capacity`) (`self.Spawned rounds`) false false null) ; Spawn and attach magazine on begin play
  ;[0 0 0] Bind weapon fired events
  (add `self.Weapon fired` (delegate `Weapon fired_Event`))
  ;[0 0 0] Bind events so hand is released when charging handle collision overlap ends
  (add `self.Charging handle overlap end` (`|CreateDelegate` :!event `ForceReleaseHanguard`)))

(event `Weapon fired_Event`
  ;[0 0 0] Bind weapon fired events
  (`KismetSystemLibrary.K2_SetTimerDelegate` (delegate `Cartridge spent`) 8.0 false 2.0 2.0) ; cartridge cool down period - cartridge emitter has a smoke trail particle if still hot when ejected
  (set `self.Cartridge hot` true)
  (`self.spawn ejector port smoke`)
  (`SceneComponent.SetVisibility` (`self.Chamber round`) true false) ; Override parent BP and set cartridge to visible so it can be ejected
)

(event `Cartridge spent`
  ;[0 0 0] Bind weapon fired events
  (set `self.Cartridge hot` false))

(event `Round inserted`
  ;[0 0 0] Cartridge elevator insert animation
  (bind (_direction _lerp) (`Timeline|Elevator anim` :!via `PlayFromStart`)
    (:`Update`
      (`SceneComponent.K2_SetRelativeRotation` (`self.Cartridge elevator`) (`KismetMathLibrary.MakeRotator` 0.0 (`KismetMathLibrary.Lerp` 0.0 11.5 _lerp)) false false)
      (`/Game/VR_Weapons/Pawn/Blueprints/BP_MotionController.RumbleController` (`self.Primary Motion Controller BP`) "/Game/VR_Weapons/Pawn/Haptics/Haptics_single.Haptics_single" 0.4 false))))

(event `self.Single Shot`
  ;[0 0 0] Shotgun firing
  (`self.Single shot sound effects`)
  (`self.Haptics` (`self.Haptic effect single`))
  (`self.Weapon fired`)
  (`self.Report noise event to AI`) ; Make enemy aware of gunshot
  (`self.Particle Effects`) ; Muzzle flash and ejector casings
  (for _ (range 1 (+ (`self.Number of Pellets`) 1))
    (bind _point (`self.Random point in circle` (* (`KismetMathLibrary.DegTan` (`self.SpreadAngle`)) (`self.Pellet distance`))))
    (set `self.Point` _point)
    (bind _outhit (`self.Shotgun line trace`))
    (`self.Bullet decals` _outhit)
    (`self.Bullet impact sound and particles` _outhit)
    (`self.Apply physics and damage` _outhit))
  (`self.Recoil_Event`))

(event `self.ReceiveTick`
  (params (DeltaSeconds :type "Float (single-precision)"))
  (bind _primary_motion_controller_bp (`self.Primary Motion Controller BP`))
  (bind _charging_handle_controller_bp (`self.Charging handle controller BP`))
  (bind _debug_mode (`self.Debug mode`))
  (bind _charging_handle_controller_bp_2 (`self.Charging handle controller BP`))
  (bind _primary_motion_controller_bp_2 (`self.Primary Motion Controller BP`))
  (bind _charging_handle_controller_bp_3 (`self.Charging handle controller BP`))
  (bind _debug_mode_2 (`self.Debug mode`))
  (bind _charging_handle_controller_bp_4 (`self.Charging handle controller BP`))
  (bind _relativelocation_x (`KismetMathLibrary.BreakVector` (`SceneComponent.RelativeLocation` (`self.Charging handle mesh`))))
  ;[0 0 0] Reloading
  (`|ExecutionSequence`
    (:`then_0`
      (`/Engine/EditorBlueprintResources/StandardMacros.IsValid` (`self.Charging handle controller BP`) ; Has charging handle var been set through overlap event
        (:`Is Valid`
          (if (and (`|EnumEquality` (`/Game/VR_Weapons/Pawn/Blueprints/BP_MotionController.GripState` _charging_handle_controller_bp_4) "NewEnumerator2") (`PrimitiveComponent.IsOverlappingActor` (`self.Charging handle collision`) _charging_handle_controller_bp_4))
            (`|ExecutionSequence`
              (:`then_0`
                (`|ExecutionSequence`
                  (:`then_0`
                    (`/Engine/EditorBlueprintResources/StandardMacros.DoOnce` false :!label _label
                      (:`Completed`
                        (set `self.Charging Handle Grabbed` true)
                        (set `self.Fore-end reset` false)
                        (`BoxComponent.SetBoxExtent` (`self.Charging handle collision`) (15.0 5.0 5.0) true)
                        (`self.Toggle charging handle fake hand` true)
                        (`GameplayStatics.PlaySoundAtLocation` (`self.Charging handle grabbed sound effect`) (`SceneComponent.K2_GetComponentLocation` (`self.Charging handle collision`)) (struct) 1.0 1.0 0.0 "/Game/VR_Weapons/Global/Audio/Weapon_Attenuation.Weapon_Attenuation" null null)
                        (`/Engine/EditorBlueprintResources/StandardMacros.IsValid` _charging_handle_controller_bp_3
                          (:`Is Valid`
                            (`/Game/VR_Weapons/Pawn/Blueprints/BP_MotionController.RumbleController` _charging_handle_controller_bp_3 "/Game/VR_Weapons/Pawn/Haptics/Haptics_single.Haptics_single" 0.4 false) ; initial grip vibration
                            (`KismetSystemLibrary.Delay` 0.2)
                            (`/Engine/EditorBlueprintResources/StandardMacros.IsValid` _charging_handle_controller_bp_3
                              (:`Is Valid`
                                (`/Game/VR_Weapons/Pawn/Blueprints/BP_MotionController.RumbleController` _charging_handle_controller_bp_3 "/Game/VR_Weapons/Pawn/Haptics/Haptics_auto.Haptics_auto" 0.2 true) ; sliding handle vibration
                              )))))))
                  (:`then_1`
                    (goto _label_7 :!via `Reset`))))
              (:`then_1`
                (if (`self.Charging Handle Grabbed`)
                  (`|ExecutionSequence`
                    (:`then_0`
                      (`/Engine/EditorBlueprintResources/StandardMacros.DoOnce` false :!label _label_2
                        (:`Completed`
                          (`self.Set charging handle start location`))))
                    (:`then_1`
                      (bind _output_get (set `self.Current distance` (`self.Charging Handle distance`)))
                      (`|ExecutionSequence`
                        (:`then_0`
                          (`self.Fore-end velocity`) ; Measure fore-end velocity to control click sound/vibration \nand cartridge ejection speed
                        )
                        (:`then_1`
                          (if (> _output_get (`self.Charging Handle max distance`))
                            (`SceneComponent.K2_SetRelativeLocation` (`self.Charging handle mesh`) (`KismetMathLibrary.MakeVector` (`KismetMathLibrary.FClamp` (`self.Current distance`) (`self.Charging Handle max distance`) 0.0)) false false)
                            (`self.Attach/detatch Bolt to Fore-end` (< (`self.Current distance`) -4.0))
                            (if (< (`self.Current distance`) -3.0)
                              (`|ExecutionSequence`
                                (:`then_0`
                                  (goto _label_5 :!via `Reset`))
                                (:`then_1`
                                  (if (> (`self.Current distance`) (+ (`self.Charging Handle max distance`) 0.2))
                                    (`|ExecutionSequence`
                                      (:`then_0`
                                        (goto _label_6 :!via `Reset`))
                                      (:`then_1`
                                        (`|ExecutionSequence`
                                          (:`then_0`
                                            (`self.Ejector port smoke` :!label _label_3))
                                          (:`then_1`
                                            (`self.Attach cartridge to bolt`)))))
                                    (else
                                      (if (`self.is Charging Handle reset`) :!label _label_4
                                        (`/Engine/EditorBlueprintResources/StandardMacros.DoOnce` true :!label _label_5 ; reset after charging handle slides back to start location
                                          (:`Completed`
                                            (`KismetSystemLibrary.PrintString` "Retracted!" _debug_mode _debug_mode (struct :`G` 1.0 :`B` 0.020307 :`A` 1.0))
                                            (`GameplayStatics.SpawnSoundAtLocation` "/Game/VR_Weapons/Guns/Shotgun/Audio/Shotgun_cocking_bolt_close_Cue.Shotgun_cocking_bolt_close_Cue" (`SceneComponent.GetSocketLocation` (`self.Ejector mesh`) "Ejector") (struct) (`self.Fore-end Velocity Clamped` 0.6) 1.0 0.0 "/Game/VR_Weapons/Global/Audio/Small_object_Attenuation.Small_object_Attenuation" null)
                                            (`/Engine/EditorBlueprintResources/StandardMacros.IsValid` _primary_motion_controller_bp
                                              (:`Is Valid`
                                                (`/Game/VR_Weapons/Pawn/Blueprints/BP_MotionController.RumbleController` _primary_motion_controller_bp "/Game/VR_Weapons/Pawn/Haptics/Haptics_single.Haptics_single" (/ (`self.Fore-end Velocity Clamped` 0.1) 2.0) false) ; Small vibration for hand holding the weapon when the charging handle is back to rest position
                                              )
                                              (:`Is Not Valid`
                                                _))
                                            (`/Engine/EditorBlueprintResources/StandardMacros.IsValid` _charging_handle_controller_bp
                                              (:`Is Valid`
                                                (`/Game/VR_Weapons/Pawn/Blueprints/BP_MotionController.RumbleController` _charging_handle_controller_bp "/Game/VR_Weapons/Pawn/Haptics/Haptics_single.Haptics_single" (`self.Fore-end Velocity Clamped` 0.1 0.8) false) ; Vibration for hand gripping the fore-end
                                              )))))))))
                              (else
                                (goto _label_4)))
                            (else
                              (`/Engine/EditorBlueprintResources/StandardMacros.DoOnce` false :!label _label_6 ; reset after charging handle slides back to start location
                                (:`Completed`
                                  (`self.Stop Haptics`) ; Stop looping haptic effect
                                  (`GameplayStatics.SpawnSoundAtLocation` "/Game/VR_Weapons/Guns/Shotgun/Audio/Shotgun_cocking_bolt_open_Cue.Shotgun_cocking_bolt_open_Cue" (`SceneComponent.GetSocketLocation` (`self.Ejector mesh`) "Ejector") (struct) (`self.Fore-end Velocity Clamped` 0.6) 1.0 0.0 "/Game/VR_Weapons/Global/Audio/Small_object_Attenuation.Small_object_Attenuation" "/Game/VR_Weapons/Global/Audio/WeaponConcurrency.WeaponConcurrency")
                                  (`/Game/VR_Weapons/Pawn/Blueprints/BP_MotionController.RumbleController` _charging_handle_controller_bp_2 "/Game/VR_Weapons/Pawn/Haptics/Haptics_single.Haptics_single" (`self.Fore-end Velocity Clamped` 0.1 0.8) false) ; Fore-end grabbing controller click
                                  (`|ExecutionSequence`
                                    (:`then_0`
                                      (`|ExecutionSequence`
                                        (:`then_0`
                                          (`/Engine/EditorBlueprintResources/StandardMacros.IsValid` _primary_motion_controller_bp_2
                                            (:`Is Valid`
                                              (`/Game/VR_Weapons/Pawn/Blueprints/BP_MotionController.RumbleController` _primary_motion_controller_bp_2 "/Game/VR_Weapons/Pawn/Haptics/Haptics_single.Haptics_single" (/ (`self.Fore-end Velocity Clamped` 0.6) 2.0) false) ; Controller holding weapon click
                                            )
                                            (:`Is Not Valid`
                                              _))
                                          (if (`SceneComponent.IsVisible` (`self.Chamber round`))
                                            (bind _particle_system (`self.Spawn shell ejection particle`)) ; Spawn shell ejection particle effect
                                            (add `ParticleSystemComponent.OnParticleCollide` _particle_system (delegate `Collision event`))
                                            (set `self.Cartridge attached to bolt` false) ; cartridge is ejected and no longer attached
                                            (set `self.One in the chamber` false) ; Now there is no cartridge in the chamber until a new \none is loaded from the magazine
                                            (set `self.Cartridge hot` false) ; Next cartridge is not hot until weapon is fired
                                          ))
                                        (:`then_1`
                                          (`self.Load next round into chamber`) ; Load round from magazine into the chamber
                                          (if (`self.One in the chamber`)
                                            (set `self.Weapon Cocked` true) ; cock weapon so its ready for next shot
                                            (`/Game/VR_Weapons/Global/Blueprints/BP_Magazine.Remove round` (`self.Magazine`))
                                            (`SceneComponent.K2_AttachToComponent` (`self.Chamber round`) (`self.Cartridge elevator`) "Cartridge" "SnapToTarget" "SnapToTarget" "SnapToTarget" true) ; attach cartridge to the elevator
                                            (else
                                              (`SceneComponent.SetVisibility` (`self.Chamber round`) false false))))))
                                    (:`then_1`
                                      (`KismetSystemLibrary.Delay` 0.1)
                                      (`/Game/VR_Weapons/Pawn/Blueprints/BP_MotionController.RumbleController` _charging_handle_controller_bp_2 "/Game/VR_Weapons/Pawn/Haptics/Haptics_auto.Haptics_auto" 0.2 true) ; Fore-end tension
                                    )))))))))))))
            (else
              (`|ExecutionSequence`
                (:`then_0`
                  (`|ExecutionSequence`
                    (:`then_0`
                      (goto _label :!via `Reset`))
                    (:`then_1`
                      (`/Engine/EditorBlueprintResources/StandardMacros.DoOnce` true :!label _label_7
                        (:`Completed`
                          (`BoxComponent.SetBoxExtent` (`self.Charging handle collision`) (12.0 5.0 5.0) true)
                          (`self.Toggle charging handle fake hand` (`self.Handguard gripped`))
                          (set `self.Charging Handle Grabbed` false)
                          (`KismetSystemLibrary.Delay` 0.2)
                          (`PlayerController.StopHapticEffect` (`GameplayStatics.GetPlayerController` 0) (select `bool` (`|EnumEquality` (`self.Primary Hand`) "Left") :`false` "Left" :`true` "Right" :!type "EControllerHand Enum"))
                          (`KismetSystemLibrary.PrintString` "Stop haptic effect" _debug_mode_2 _debug_mode_2 (struct :`R` 1.0 :`G` 0.307249 :`A` 1.0)))))))
                (:`then_1`
                  (goto _label_2 :!via `Reset`))
                (:`then_2`
                  (if (not (`self.Fore-end reset`)) :!label _label_8
                    (if (`self.is Charging Handle reset`)
                      (set `self.Fore-end reset` true)
                      (goto _label_5)
                      (elif (not (`self.Charging Handle Grabbed`))
                        (`SceneComponent.K2_SetRelativeLocation` (`self.Charging handle mesh`) (`KismetMathLibrary.MakeVector` (`KismetMathLibrary.FInterpTo_Constant` _relativelocation_x 0.0 DeltaSeconds 185.0)) false false) ; Slide back to start location when grip is released
                        (`self.Fore-end velocity`)))))))))
        (:`Is Not Valid`
          (goto _label_8))))
    (:`then_1`
      (`self.Gun aiming`))))

(event `spawn ejector port smoke`
  ;[0 0 0] Reloading
  (goto _label_3 :!via `Do once Reset`))

(event `Collision event`
  (params (EventName :type Name) (EmitterTime :type "Float (double-precision)") (ParticleTime :type Integer) (Location :type "Vector Structure") (Velocity :type "Vector Structure") (Direction :type "Vector Structure") (Normal :type "Vector Structure") (BoneName :type Name) (PhysMat :type "PhysicalMaterial Object Reference"))
  ;[0 0 0] Reloading
  (`/Engine/EditorBlueprintResources/StandardMacros.DoOnce` false :!label _label_9
    (:`Completed`
      (`GameplayStatics.PlaySoundAtLocation` (select `EPhysicalSurface` (`PhysicalMaterial.SurfaceType` PhysMat) :`SurfaceType_Default` "/Game/VR_Weapons/Guns/Shotgun/Audio/Shotgun_shell_drop_01_Cue.Shotgun_shell_drop_01_Cue" :`SurfaceType1` "/Game/VR_Weapons/Guns/Shotgun/Audio/Shotgun_shell_drop_01_Cue.Shotgun_shell_drop_01_Cue" :`SurfaceType3` "/Game/VR_Weapons/Guns/Shotgun/Audio/Shotgun_shell_drop_01_Cue.Shotgun_shell_drop_01_Cue" :!type "SoundBase Object Reference") Location (struct) 1.0 1.0 0.0 "/Game/VR_Weapons/Global/Audio/Small_object_Attenuation.Small_object_Attenuation" null null) ; shell drop sound effect
      (`KismetSystemLibrary.Delay` 1.5)
      (goto _label_9 :!via `Reset`))))

(fn `Align mesh particle rotation with weapon`
  (params (InRot :type "Rotator Structure"))
  (returns (rotation :type "Float (double-precision)"))
  (bind _yaw (.yaw InRot))
  (return (/ (+ (select `bool` (< _yaw 0.0) :`true` 360.0 :!type "Float (single-precision)") _yaw) 360.0)))

(fn `Attach cartridge to bolt`
  (bind _debug_mode (`self.Debug mode`))
  (if (and (> (`self.Current distance`) -10.0) (not (`self.Cartridge attached to bolt`)) (`SceneComponent.IsVisible` (`self.Chamber round`)))
    (bind _returnvalue (`SceneComponent.K2_AttachToComponent` (`self.Chamber round`) (`self.Ejector mesh`) "Ejector" "SnapToTarget" "SnapToTarget" "SnapToTarget" true))
    (if _returnvalue
      (set `self.Cartridge attached to bolt` true)
      (`KismetSystemLibrary.PrintString` "Cartridge attached to bolt" _debug_mode _debug_mode (struct :`R` 0.088293 :`G` 1.0 :`A` 1.0) 5.0))))

(fn `Attach/detatch Bolt to Fore-end`
  (params (attach :type Boolean))
  (if attach
    (if (not (`self.Bolt attached to fore-end`))
      (bind _returnvalue (`SceneComponent.K2_AttachToComponent` (`self.Ejector mesh`) (`self.Charging handle mesh`) "None" "KeepWorld" "KeepWorld" "KeepWorld" true)) ; Attach bolt to fore-end
      (set `self.Bolt attached to fore-end` _returnvalue))
    (elif (`self.Bolt attached to fore-end`)
      (bind _returnvalue_2 (`SceneComponent.K2_AttachToComponent` (`self.Ejector mesh`) (`self.Gun mesh`) "None" "KeepWorld" "KeepWorld" "KeepWorld" true)) ; Detatch bolt from fore-end
      (set `self.Bolt attached to fore-end` (not _returnvalue_2)) ; bolt is no longer attached to fore-end
      (`SceneComponent.K2_SetRelativeLocation` (`self.Ejector mesh`) (0.0 0.0 0.0) false false))))

(fn `ForceReleaseHanguard`
  (bind _secondary_motion_controller_bp (`self.Secondary Motion Controller BP`))
  (if (and (`KismetSystemLibrary.IsValid` _secondary_motion_controller_bp) (`self.Handguard gripped`))
    (set `self.Handguard gripped` false)
    (set `/Game/VR_Weapons/Pawn/Blueprints/BP_MotionController.Weapon` "NewEnumerator0" _secondary_motion_controller_bp)
    (`SceneComponent.SetVisibility` (`/Game/VR_Weapons/Pawn/Blueprints/BP_MotionController.HandMesh` _secondary_motion_controller_bp) true true)
    (`SceneComponent.SetVisibility` (`self.Charging handle grip`) false false)
    (`PlayerController.StopHapticEffect` (`GameplayStatics.GetPlayerController` 0) (`/Game/VR_Weapons/Pawn/Blueprints/BP_MotionController.Hand` _secondary_motion_controller_bp))
    (`self.Reset hand rotation`)))

(fn `Fore-end Velocity Clamped`
  (params (Min :type "Float (double-precision)" :default 0.6) (Max :type "Float (double-precision)" :default 1.0))
  (returns (ReturnValue :type "Float (double-precision)"))
  (return (`KismetMathLibrary.FClamp` (`self.Fore-end velocity normalized`) Min Max)))

(fn `GripHandGuard`
  (params (Hand :type "/Game/VR_Weapons/Pawn/Blueprints/BP_MotionController Object Reference"))
  (returns (HandguardGrabbed :type Boolean))
  (bind _hand (`local.Hand`))
  (if (and (`PrimitiveComponent.IsOverlappingActor` (`self.Charging handle collision`) Hand) (!= (`self.Primary Motion Controller BP`) null))
    (set `self.Handguard gripped` true)
    (`/Game/VR_Weapons/Pawn/Blueprints/BP_MotionController.RumbleController` _hand "/Game/VR_Weapons/Pawn/Haptics/Haptics_single.Haptics_single" 0.4 false)
    (set `self.Secondary Motion Controller BP` _hand)
    (set `/Game/VR_Weapons/Pawn/Blueprints/BP_MotionController.Weapon` (`self.Weapon`) _hand)
    (`SceneComponent.SetVisibility` (`/Game/VR_Weapons/Pawn/Blueprints/BP_MotionController.HandMesh` _hand) false true) ; Hide motion controller hand mesh
    (`SceneComponent.SetVisibility` (`self.Charging handle grip`) true false) ; Show fore-end hand
    (return (`self.Handguard gripped`))))

(fn `Handguard release`
  (params (Hand :type "Object Object Reference"))
  (bind _secondary_motion_controller_bp (`self.Secondary Motion Controller BP`))
  (bind _debug_mode (`self.Debug mode`))
  (if (and (== Hand _secondary_motion_controller_bp) (`KismetSystemLibrary.IsValid` _secondary_motion_controller_bp) (`self.Handguard gripped`))
    (set `/Game/VR_Weapons/Pawn/Blueprints/BP_MotionController.Weapon` "NewEnumerator0" _secondary_motion_controller_bp)
    (`SceneComponent.SetVisibility` (`/Game/VR_Weapons/Pawn/Blueprints/BP_MotionController.HandMesh` _secondary_motion_controller_bp) true true)
    (`SceneComponent.SetVisibility` (`self.Charging handle grip`) false false)
    (`SceneComponent.SetVisibility` (`self.HandGuardGrabbingHand`) false false)
    (`PlayerController.StopHapticEffect` (`GameplayStatics.GetPlayerController` 0) (`/Game/VR_Weapons/Pawn/Blueprints/BP_MotionController.Hand` _secondary_motion_controller_bp))
    (`self.Reset hand rotation`)
    (set `self.Secondary Motion Controller BP` null) ; clear reference to secondary motion controller
    (set `self.Handguard gripped` false)
    (`KismetSystemLibrary.PrintString` "hand guard released" _debug_mode _debug_mode (struct :`R` 0.159835 :`G` 1.0 :`A` 1.0))))

(fn `LineTraceFromBarrel`
  (returns (OutHit :type "HitResult Structure"))
  (bind _outhit (`parent.LineTraceFromBarrel`))
  (return _outhit))

(fn `Pellet spread test`
  (for _ (range 1 (+ (`self.Number of Pellets`) 1))
    (bind _point (`self.Random point in circle` (* (`KismetMathLibrary.DegTan` (`self.SpreadAngle`)) (`self.Pellet distance`))))
    (set `self.Point` _point)
    (`self.Shotgun line trace`))
  (set `self.Test pellet spread` false))

(fn `Random point in circle`
  (params (Radius :type "Float (double-precision)"))
  (returns (Point :type "Vector2D Structure"))
  (locals (Angle :type "Float (double-precision)") (`Distance from center` :type "Float (double-precision)"))
  (set `local.Angle` (`KismetMathLibrary.RandomFloatInRange` 0.0 360.0))
  (set `local.Distance from center` (`KismetMathLibrary.RandomFloatInRange` 0.0 (* (`local.Radius`) (`CurveFloat.GetFloatValue` (`self.PelletSpreadCurve`) (`KismetMathLibrary.RandomFloatInRange` 0.0 1.0)))))
  (return (`KismetMathLibrary.MakeVector2D` (* (`local.Distance from center`) (`KismetMathLibrary.DegCos` (`local.Angle`))) (* (`local.Distance from center`) (`KismetMathLibrary.DegSin` (`local.Angle`))))))

(fn `Ready to fire`
  (returns (`Round in the chamber` :type Boolean))
  ;[0 0 0] Override parent function
  (if (`self.Fore-end reset`)
    (bind _round_in_the_chamber (`parent.Ready to fire`))
    (return _round_in_the_chamber)))

(fn `Shotgun line trace`
  (returns (OutHit :type "HitResult Structure"))
  (bind _gun_mesh (`self.Gun mesh`))
  (bind _returnvalue (`SceneComponent.GetSocketLocation` _gun_mesh "Barrel"))
  (bind (_x _y) (`KismetMathLibrary.BreakVector2D` (`self.Point`)))
  (bind _returnvalue_2 (`SceneComponent.GetSocketRotation` _gun_mesh "Barrel"))
  (bind _outhit (`KismetSystemLibrary.LineTraceSingle` :`Start` _returnvalue :`End` (+ (+ _returnvalue (* (`KismetMathLibrary.GetForwardVector` _returnvalue_2) (`self.Pellet distance`))) (* (`KismetMathLibrary.GetRightVector` _returnvalue_2) _x) (* (`KismetMathLibrary.GetUpVector` _returnvalue_2) _y)) :`TraceChannel` "TraceTypeQuery1" :`DrawDebugType` (select `bool` (`self.Debug mode`) :`true` "ForDuration" :!type "EDrawDebugTrace Enum") :`DrawTime` 1.0))
  (return _outhit))

(fn `Spawn shell ejection particle`
  (returns (`Particle system` :type "ParticleSystemComponent Object Reference"))
  (bind _fore_end_velocity_normalized (`self.Fore-end velocity normalized`))
  (bind _debug_mode (`self.Debug mode`))
  (bind (_returnvalue_location _returnvalue_rotation) (`KismetMathLibrary.BreakTransform` (`SceneComponent.GetSocketTransform` (`self.Gun mesh`) "Ejector" "RTS_World")))
  (bind _returnvalue (`GameplayStatics.SpawnEmitterAtLocation` (select `bool` (`self.Cartridge hot`) :`false` "/Game/VR_Weapons/Guns/Shotgun/Particles/P_Shotgun_casing_ejections.P_Shotgun_casing_ejections" :`true` "/Game/VR_Weapons/Guns/Shotgun/Particles/P_Shotgun_casing_ejections_hot.P_Shotgun_casing_ejections_hot" :!type "ParticleSystem Object Reference") _returnvalue_location _returnvalue_rotation)) ; Casing ejection particle emitter
  (`FXSystemComponent.SetVectorParameter` _returnvalue "Mesh Rot" (`KismetMathLibrary.MakeVector` 0.0 0.0 (`self.Align mesh particle rotation with weapon` _returnvalue_rotation))) ; Orient mesh particle rotation correctly
  (`KismetSystemLibrary.PrintString` (`KismetStringLibrary.Concat_StrStr` "Fore-end velocity" (`KismetStringLibrary.Conv_DoubleToString` _fore_end_velocity_normalized)) _debug_mode _debug_mode (struct :`R` 0.194859 :`G` 1.0 :`A` 1.0) 7.0)
  (`FXSystemComponent.SetVectorParameter` _returnvalue "Casing velocity" (`KismetMathLibrary.VLerp` (5.0 75.0 15.0) (10.0 225.0 45.0) _fore_end_velocity_normalized))
  (return _returnvalue))

(fn `UserConstructionScript`
  (`parent.UserConstructionScript`)
  (`ActorComponent.K2_DestroyComponent` (`self.Safety mesh`))
  ;[0 0 0] Debugging
  (if (`self.Test pellet spread`)
    (if (`self.Debug mode`)
      (`KismetSystemLibrary.FlushPersistentDebugLines` :!label _label)
      (`self.Pellet spread test`)
      (else
        (`|ExecutionSequence`
          (:`then_0`
            (set `self.Debug mode` true)
            (goto _label))
          (:`then_1`
            (set `self.Debug mode` false)))))
    (else
      (`KismetSystemLibrary.FlushPersistentDebugLines`))))